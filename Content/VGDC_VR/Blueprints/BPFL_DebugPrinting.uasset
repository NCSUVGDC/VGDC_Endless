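; Blueprint function library for formatted on-screen debug printing in the VR project.
; PrintDebug is gated by a bool and maps four severity levels to prefix, color and duration, with errors also getting a suffix.
; It prints the message in quotes after the invoking object's display name.
; Helper functions format ints, floats and int ranges as optionally named bracketed strings, using parentheses for exclusive ranges.
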(fn `Add Space After Name If Valid`
  (params (Name :type String))
  (returns (Formatted :type String))
  ;[1 0.3224 0.3124] Empty string?
  (if (== (`KismetStringLibrary.Len` Name) 0)
    ;[0.3364 1 0.315] Name empty; return blank
    (return "")
    (else
      ;[0.3209 0.7662 1] Name not empty; add space after
      (return (`KismetStringLibrary.Concat_StrStr` (`local.Name`) ": ")))))

(fn `Debug Format Float`
  (params (Name :type String) (Float :type "Float (double-precision)") (Decimals :type Integer :default 2))
  (returns (String :type String))
  (locals (Prefix :type String))
  (return (`KismetStringLibrary.Concat_StrStr` (`self.Add Space After Name If Valid` Name) "[" (`KismetTextLibrary.Conv_TextToString` (`KismetTextLibrary.Conv_DoubleToText` Float "HalfFromZero" false 1 324 0 Decimals)) "]")))

(fn `Debug Format Int`
  (params (Name :type String) (Integer :type Integer))
  (returns (String :type String))
  (locals (Prefix :type String))
  (return (`KismetStringLibrary.Concat_StrStr` (`self.Add Space After Name If Valid` Name) "[" (`KismetStringLibrary.Conv_IntToString` Integer) "]")))

(fn `Debug Format Int Range`
  (params (Name :type String) (Min :type Integer) (Max :type Integer) (Inclusive :type Boolean :default true))
  (returns (String :type String))
  (if Inclusive
    ;[1 1 1] Inclusive is [x, y]
    (return (`KismetStringLibrary.Concat_StrStr` (`self.Add Space After Name If Valid` (`local.Name`)) "[" (`KismetStringLibrary.Conv_IntToString` (`local.Min`)) ", " (`KismetStringLibrary.Conv_IntToString` (`local.Max`)) "]"))
    (else
      ;[1 1 1] Exclusive is (x, y)
      (return (`KismetStringLibrary.Concat_StrStr` (`self.Add Space After Name If Valid` (`local.Name`)) "(" (`KismetStringLibrary.Conv_IntToString` (`local.Min`)) ", " (`KismetStringLibrary.Conv_IntToString` (`local.Max`)) ")")))))

(fn `Print Debug`
  (params (Message :type String) (`Can Print` :type Boolean :default true) (Severity :type "/Game/VGDC_VR/Blueprints/DebugSeverity Enum" :default "NewEnumerator4") (Invoker :type "Actor Object Reference"))
  (locals (Prefix :type String) (Suffix :type String) (Color :type "LinearColor Structure") (Duration :type "Float (double-precision)"))
  (if `Can Print`
    (`|ExecutionSequence`
      (:`then_0`
        ;[0.894 1 0.2379] Set display parameters based on severity
        (switch `/Game/VGDC_VR/Blueprints/DebugSeverity` Severity
          (:`NewEnumerator4`
            (set `local.Prefix` "[Verbose]")
            (set `local.Color` (struct :`R` 0.65625 :`G` 0.65625 :`B` 0.65625 :`A` 1.0))
            (set `local.Duration` 2.0))
          (:`NewEnumerator0`
            (set `local.Prefix` "[Log]")
            (set `local.Color` (struct :`R` 0.101563 :`G` 0.8125 :`B` 0.129377 :`A` 1.0))
            (set `local.Duration` 4.0))
          (:`NewEnumerator1`
            (set `local.Prefix` "[Notice]")
            (set `local.Color` (struct :`R` 0.911458 :`G` 0.487622 :`B` 0.099927 :`A` 1.0))
            (set `local.Duration` 6.0))
          (:`NewEnumerator2`
            (set `local.Prefix` "### ERROR ###")
            (set `local.Suffix` "### ###")
            (set `local.Color` (struct :`R` 0.911458 :`B` 0.009066 :`A` 1.0))
            (set `local.Duration` 8.0))))
      (:`then_1`
        ;[0.5212 0.4969 1] Actual Printing
        (`KismetSystemLibrary.PrintString` (`local.Invoker`) (`KismetStringLibrary.Concat_StrStr` (`local.Prefix`) " " (`KismetSystemLibrary.GetDisplayName` (`local.Invoker`)) ": \"" (`local.Message`) "\" " (`local.Suffix`)) true true (`local.Color`) (`local.Duration`))))))