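; ScoreKeeping_BP is a score-keeping Blueprint that sets up and loads the game's high-score leaderboard from a file.
; On BeginPlay it builds default named entries with descending scores if no file exists, passes HighScores to AddHighScores, then calls GetHighScores.
; File access and entry creation come from functions defined outside this graph.
; PrintAllScores is an uncalled debug helper here, and OnGameOver is an empty event.
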(event `self.ReceiveBeginPlay`
  (bind _filename (`self.filename`))
  (`self.MakeDefaultHighScores`)
  (`self.AddHighScores` _filename (`self.highScores`))
  (`self.GetHighScores` _filename))

(event `OnGameOver`)

(fn `MakeDefaultHighScores`
  (locals (defaultNames :type "Array of String") (scores :type "Map of String to Object Object Reference"))
  (bind _returnvalue (`self.bFileExists` (`self.filename`)))
  (if _returnvalue
    (`KismetSystemLibrary.PrintString` "File Exists")
    (else
      (for _index (range (`self.leaderboardMax`))
        (`KismetArrayLibrary.Array_Add` (`self.highScores`) (`self.CreateLeaderboardEntry` (`|GetArrayItem` (`local.defaultNames`) _index) (* (- (`self.leaderboardMax`) _index) 75))))
      (return))))

(fn `PrintAllScores`
  (params (HighScores :type "Array of ScoreContainer Object Reference"))
  (for _index (range (`KismetArrayLibrary.Array_Length` HighScores))
    (`KismetSystemLibrary.PrintString` (`ScoreContainer.ToString` (`|GetArrayItem` (`self.highScores`) _index)))))

(fn `UserConstructionScript`)