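; BlastDoor is a VR project actor that builds a ring of pooled cell actors when play begins; no door movement or opening logic is present.
; SpawnCells spaces SpawnCount actors evenly by angle on a circle of the given Radius, using sine and cosine in the world YZ plane around the actor's location.
; Each comes from Pooler with the same fixed rotation, so the ring ignores the actor's own rotation.
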(event `self.ReceiveBeginPlay`
  (`self.SpawnCells`))

(fn `SpawnCells`
  (locals (percentage :type "Float (double-precision)"))
  (bind _radius (`self.radius`))
  (for _index (range (`self.spawnCount`))
    (bind _output_get (set `local.percentage` (/ (`KismetMathLibrary.Conv_IntToDouble` _index) (`KismetMathLibrary.Conv_IntToDouble` (`self.spawnCount`)))))
    (bind _returnvalue (* 360 _output_get))
    (`/Game/VGDC_VR/Environment/Technical/ObjectPooler_BP.createActor` (`self.pooler`) (+ (`KismetMathLibrary.MakeVector` 0.0 (* (`KismetMathLibrary.DegSin` _returnvalue) _radius) (* _radius (`KismetMathLibrary.DegCos` _returnvalue))) (`self.K2_GetActorLocation`)) (struct :`Pitch` 90.0))))

(fn `UserConstructionScript`)