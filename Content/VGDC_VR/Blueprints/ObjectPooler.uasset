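; Object pool actor for the VR project that manages reusable instances of a poolable actor class, running pool creation on BeginPlay.
; CreateActor reuses a hidden instance or spawns one up to a maximum size, then moves it to the requested position.
; ActivityToggle switches visibility, tick and collision together, with the hidden flag marking inactive objects.
; ShrinkPool destroys the first inactive instance, but nothing in this graph calls it.
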(event `self.ReceiveBeginPlay`
  (`self.createPool`))

(event `self.ReceiveTick`
  (params (DeltaSeconds :type "Float (single-precision)")))

(fn `activityToggle`
  (params (obj :type "Actor Object Reference") (active :type Boolean))
  (locals (hideToggle :type Boolean :default false) (collisionToggle :type Boolean :default true) (tickerToggle :type Boolean :default true))
  (if active
    (set `local.hideToggle` false)
    (else
      (set `local.hideToggle` true)))
  (if active
    (set `local.tickerToggle` true)
    (else
      (set `local.tickerToggle` false)))
  (if active
    (set `local.collisionToggle` true)
    (else
      (set `local.collisionToggle` false)))
  (`self.SetActorHiddenInGame` obj (`local.hideToggle`))
  (`self.SetActorTickEnabled` obj (`local.tickerToggle`))
  (`self.SetActorEnableCollision` obj (`local.collisionToggle`)))

(fn `anyObjectsInactive`
  (returns (anyInactive :type Boolean))
  (locals (inactive :type Boolean))
  (bind _objpool (`self.objPool`))
  (for _index (range (+ (`KismetArrayLibrary.Array_Length` _objpool) 1))
    (if (`Actor.bHidden` (`|GetArrayItem` _objpool _index))
      (bind _output_get (set `local.inactive` true))
      (return _output_get)))
  (return _output_get))

(fn `createActor`
  (params (position :type "Vector Structure"))
  (returns (pooledObj :type "Actor Object Reference"))
  (locals (anyInactive :type Boolean) (count :type Integer) (obj :type "Actor Object Reference"))
  (bind _obj (`local.obj`))
  (bind _objpool (`self.objPool`))
  (bind _output (`|GetArrayItem` (`self.objPool`)))
  ;[1 0 0] Look through entire object pool for any inactive objects
  (while (< (`local.count`) (`self.currentPoolSize`))
    (if (`Actor.bHidden` (`|GetArrayItem` (`self.objPool`)))
      (set `local.anyInactive` true))
    (set `local.count` (+ (`local.count`) 1)))
  ;[0.8646 0.709 0] Are there any inactive objects in the pool?
  (if (`local.anyInactive`)
    (set `local.count` 0)
    ;[0.009825 0.9583 0.1795] Search for the first inactive instance within the pool and set reference to it
    (while (== (`local.obj`) null)
      (if (`Actor.bHidden` _output)
        (set `local.obj` _output))
      (set `local.count` (+ (`local.count`) 1)))
    (`self.K2_SetActorLocation` _obj position false false :!label _label) ; Set Pooled Object's location
    (else
      ;[0.08778 1 0.9003] If not, is the current pool size less than its maximum capacity? (maxSize)
      (if (< (`self.currentPoolSize`) (`self.maxSize`))
        ;[0 0.01656 0.3125] Spawn a new instance if there are no objects in the pool that are inactive
        (bind _returnvalue (`|SpawnActorFromClass` "/Game/VGDC_VR/Blueprints/PoolableObject.PoolableObject_C" (`self.GetTransform`) "Undefined" "OverrideRootScale" null null))
        (set `local.obj` _returnvalue)
        ;[1 0 0.2166] Add new instance to the pool and update pool size variable
        (`KismetArrayLibrary.Array_Add` _objpool _obj)
        (set `self.currentPoolSize` (`KismetArrayLibrary.Array_Length` _objpool))
        (goto _label)
        (else
          (`KismetSystemLibrary.PrintString` "Error! Current Pool has reached it's current limit!")))))
  (return _obj))

(fn `createPool`
  ;[1 0 0] Creates a pool of Actors, with the count being equal the mininum pool size (minSize)
  (for _ (range (+ (`self.minSize`) 1))
    (bind _pooledobj (`self.createActor` (0.0 0.0 0.0)))
    (`self.activityToggle` _pooledobj) ; Set each object in pool inactive
  ))

(fn `deleteActor`
  (params (object :type "Actor Object Reference"))
  (bind _objpool (`self.objPool`))
  ;[1 0 0] Removes actor from object pool, destroys it, and proceeds to update pool size variable (currentPoolSize)
  (`KismetArrayLibrary.Array_RemoveItem` _objpool object)
  (`self.K2_DestroyActor` object)
  (set `self.currentPoolSize` (`KismetArrayLibrary.Array_Length` _objpool)))

(fn `findFirstInactive`
  (returns (object :type "Actor Object Reference"))
  (bind _objpool (`self.objPool`))
  ;[0.8646 0.709 0] Returns the first inactive instance in the object pool
  (for _index (range (+ (`KismetArrayLibrary.Array_Length` _objpool) 1))
    (bind _output (`|GetArrayItem` _objpool _index))
    (if (`Actor.bHidden` _output)
      (return _output)))
  (return _output))

(fn `shrinkPool`
  ;[0 0.01656 0.3125] Checks if any objects are inactive within the pool, and deletes the first instance
  (if (`self.anyObjectsInactive`)
    (`self.deleteActor` (`self.findFirstInactive`))))

(fn `UserConstructionScript`)