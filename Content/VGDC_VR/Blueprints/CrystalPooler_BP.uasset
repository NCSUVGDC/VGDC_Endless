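; CrystalPooler_BP is an actor pooler that places crystals at random positions within set bounds.
; Its only active logic, SpawnWithinBounds, calls CreateActor with zero rotation and returns the resulting actor.
; The position randomizes X and Z within plus or minus Radius, giving a square area, and feeds ZOffset into Y despite the name.
; Event graph and construction script run no logic.
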(fn `SpawnWithinBounds`
  (returns (pooledObj :type "Actor Object Reference"))
  (bind _radius (`self.radius`))
  (bind _returnvalue (`KismetMathLibrary.RandomFloatInRange` (* -1 _radius) _radius))
  (bind _pooledobj (`self.createActor` (`KismetMathLibrary.MakeVector` _returnvalue (`self.zOffset`) _returnvalue)))
  (return _pooledobj))

(fn `UserConstructionScript`)