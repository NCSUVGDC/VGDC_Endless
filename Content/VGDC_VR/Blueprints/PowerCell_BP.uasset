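; Power cell actor for a VR game that displays as red, green, blue or yellow.
; ChangePowerCell creates the mesh component at runtime if needed and swaps in the static mesh matching the Color value, starting at BeginPlay.
; SetColor applies a given color, while the ChangeColor event steps through the four colors with a wrapping Index, both refreshing the mesh through ChangePowerCell.
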(event `self.ReceiveBeginPlay`
  (`self.ChangePowerCell`))

(event `ChangeColor`
  (bind _index (`self.index`))
  (switch `int` (`self.index`)
    (:`Default`
      (set `self.Color` "VE_RED" :!label _label))
    (:`0`
      (goto _label))
    (:`1`
      (set `self.Color` "VE_GREEN"))
    (:`2`
      (set `self.Color` "VE_BLUE"))
    (:`3`
      (set `self.Color` "VE_YELLOW")))
  (if (< _index 3)
    (set `self.index` (+ _index 1))
    (else
      (set `self.index` 0)))
  (`self.ChangePowerCell`))

(fn `ChangePowerCell`
  (bind _powercellmesh (`self.powerCellMesh`))
  (if (== (`self.powerCellMesh`) null)
    (bind _returnvalue (`AddComponent|NODE_AddStaticMeshComponent-1`))
    (set `self.powerCellMesh` _returnvalue))
  (switch `EColorsEnum` (`self.Color`)
    (:`VE_RED`
      (`StaticMeshComponent.SetStaticMesh` _powercellmesh "/Game/Meshes/PowerCell_StaticMesh_RED.PowerCell_StaticMesh_RED"))
    (:`VE_GREEN`
      (`StaticMeshComponent.SetStaticMesh` _powercellmesh "/Game/Meshes/PowerCell_StaticMesh_GREEN.PowerCell_StaticMesh_GREEN"))
    (:`VE_BLUE`
      (`StaticMeshComponent.SetStaticMesh` _powercellmesh "/Game/Meshes/PowerCell_StaticMesh_BLUE.PowerCell_StaticMesh_BLUE"))
    (:`VE_YELLOW`
      (`StaticMeshComponent.SetStaticMesh` _powercellmesh "/Game/Meshes/PowerCell_StaticMesh_YELLOW.PowerCell_StaticMesh_YELLOW"))))

(fn `SetColor`
  (params (color :type "EColorsEnum Enum" :default "VE_RED"))
  (set `self.Color` color)
  (`self.ChangePowerCell`))

(fn `UserConstructionScript`)