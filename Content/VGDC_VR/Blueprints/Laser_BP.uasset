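; Laser Blueprint actor that slides once from its starting position to an offset end point over a set duration.
; BeginPlay caches the root's world location as the origin, with EndPoint treated as an offset from it.
; Tick accumulates elapsed time and, while within TranslationTime, calls Translate to lerp the actor's location without sweep.
; It has no looping, overlap response or construction logic.
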(event `self.ReceiveBeginPlay`
  (set `self.origin` (`SceneComponent.K2_GetComponentLocation` (`self.DefaultSceneRoot`))))

(event `self.ReceiveTick`
  (params (DeltaSeconds :type "Float (single-precision)"))
  (bind _translationtime (`self.translationTime`))
  (bind _origin (`self.origin`))
  (bind _output_get (set `self.translationTimer` (+ DeltaSeconds (`self.translationTimer`))))
  (if (<= _output_get _translationtime)
    (`self.Translate` _origin (+ _origin (`self.endPoint`)) (/ _output_get _translationtime))))

(fn `Translate`
  (params (startPoint :type "Vector Structure") (endPoint :type "Vector Structure") (delta :type "Float (double-precision)"))
  (`self.K2_SetActorLocation` (`KismetMathLibrary.VLerp` startPoint endPoint delta)))

(fn `UserConstructionScript`)