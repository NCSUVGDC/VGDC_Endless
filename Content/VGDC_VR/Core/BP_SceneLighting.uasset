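; BP_SceneLighting controls scene-wide fade-out and fade-in through the post-process settings of AmbientLighting.
; A single Fade timeline drives color saturation and scales intensity from its default value by a brightness track.
; FadeOut plays the timeline from the start and FadeIn reverses it from the end.
; The construction script sets the timeline play rate to the inverse of FadeTime, so that variable controls fade duration.
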(event `Fade Out`
  (bind (_direction _brightness _saturation) (`Timeline|Fade` :!via `PlayFromStart` :!label _label)
    (:`Update`
      (setmembers `PostProcessSettings` :`StructRef` (`PostProcessComponent.Settings` (`self.Ambient Lighting`)) :`ColorSaturation` (`KismetMathLibrary.MakeVector4` _saturation _saturation _saturation _saturation) :`AmbientCubemapIntensity` (* (`self.Default Lighting Intensity`) _brightness)))))

(event `Fade In`
  (goto _label :!via `ReverseFromEnd`))

(fn `UserConstructionScript`
  (`TimelineComponent.SetPlayRate` (`self.Fade`) (/ 1.0 (`self.Fade Time`))))