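; Game state for a VR tunnel game, running the flow from hub through door approach and play to game over.
; BeginPlay passes itself to interested actors via an interface, caches key scene actors and starts hub music.
; Tick updates level stats from the tunnel manager and, per state, darkens crystals, moves platform and player doorward while brightening them, or slides the hub back.
; It also switches music and computes total score from level and weapon stats.
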(event `self.ReceiveBeginPlay`
  ;[1 1 1] Notify all actors who need BP Base Game State
  (bind _outactors (`GameplayStatics.GetAllActorsWithInterface` "/Game/VGDC_VR/Core/BPI_NeedsGameState.BPI_NeedsGameState_C"))
  (for _array_element _outactors
    (message `/Game/VGDC_VR/Core/BPI_NeedsGameState.Set BP_BaseGameState` _array_element self))
  (`|ExecutionSequence`
    (:`then_0`
      ;[1 1 1] Get Lighting
      (bind _outactors_2 (`GameplayStatics.GetAllActorsOfClass` "/Game/VGDC_VR/Environment/Lighting/BP_SceneLighting.BP_SceneLighting_C"))
      (set `self.Scene Lighting` (`|GetArrayItem` _outactors_2)))
    (:`then_1`
      ;[1 1 1] Get Platform
      (bind _outactors_3 (`GameplayStatics.GetAllActorsOfClass` "/Game/VGDC_VR/Environment/Platform/BP_Platform.BP_Platform_C"))
      (set `self.Platform` (`|GetArrayItem` _outactors_3))
      ;[1 1 1] Get Hub Platform
      (bind _outactors_4 (`GameplayStatics.GetAllActorsOfClass` "/Game/VGDC_VR/Environment/Hub/BP_HubPlatform.BP_HubPlatform_C"))
      (set `self.Hub Rails` (`|GetArrayItem` _outactors_4)))
    (:`then_2`
      ;[1 1 1] Get Hub
      (bind _outactors_5 (`GameplayStatics.GetAllActorsOfClass` "/Game/VGDC_VR/Environment/Hub/BP_HubWalls.BP_HubWalls_C"))
      (set `self.Hub` (`|GetArrayItem` _outactors_5)))
    (:`then_3`
      ;[1 1 1] Get Hub
      (bind _outactors_6 (`GameplayStatics.GetAllActorsOfClass` "/Game/VGDC_VR/Core/BP_ScoreKeeping.BP_ScoreKeeping_C"))
      (set `self.Scorekeeping` (`|GetArrayItem` _outactors_6)))
    (:`then_4`
      ;[1 1 1] Spawn Music
      (`self.Change Music` (`self.Music - Hub`)))))

(event `self.ReceiveTick`
  (params (DeltaSeconds :type "Float (single-precision)"))
  (bind _returnvalue (* (`GameplayStatics.GetWorldDeltaSeconds`) (`/Game/VGDC_VR/Environment/Platform/BP_Platform.Hub Movement Speed` (`self.Platform`))))
  (bind _returnvalue_2 (`KismetMathLibrary.MakeVector` 0.0 (* (`/Game/VGDC_VR/Environment/Technical/BP_TunnelManager.Current Hall Speed` (`self.Tunnel Manager`)) (`GameplayStatics.GetWorldDeltaSeconds`))))
  (`self.Update Level Stats`)
  (switch `/Game/VGDC_VR/Core/GamePlayState` (`self.Game State`)
    (:`NewEnumerator4`
      (`KismetMaterialLibrary.SetScalarParameterValue` "/Game/VGDC_VR/Materials/M_GlobalLightDimming.M_GlobalLightDimming" "Brightness" 0.0))
    (:`NewEnumerator5`
      (if (< (`self.Platform Transition Distance Covered`) (`self.Hub Door Distance`))
        (`|ExecutionSequence`
          (:`then_0`
            (set `self.Platform Transition Distance Covered` (+ (`self.Platform Transition Distance Covered`) _returnvalue))
            (`self.K2_AddActorWorldOffset` (`self.Platform`) (`KismetMathLibrary.MakeVector` 0.0 (* _returnvalue -1.0)) false false)
            (`self.K2_AddActorWorldOffset` (`self.Player Pawn`) (`KismetMathLibrary.MakeVector` 0.0 (* _returnvalue -1.0)) false false))
          (:`then_1`
            (`KismetMaterialLibrary.SetScalarParameterValue` "/Game/VGDC_VR/Materials/M_GlobalLightDimming.M_GlobalLightDimming" "Brightness" (`KismetMathLibrary.MultiplyMultiply_FloatFloat` (/ (`self.Platform Transition Distance Covered`) (`self.Hub Door Distance`)) 6.0))))
        (else
          (`self.Start Game`)
          (`KismetMaterialLibrary.SetScalarParameterValue` "/Game/VGDC_VR/Materials/M_GlobalLightDimming.M_GlobalLightDimming" "Brightness" 1.0))))
    (:`NewEnumerator0`
      (`self.K2_AddActorWorldOffset` (`self.Hub`) _returnvalue_2 false false)
      (`self.K2_AddActorWorldOffset` (`self.Hub Rails`) _returnvalue_2 false false))))

(fn `Change Music`
  (params (`New Sound` :type "SoundWave Object Reference"))
  (`AudioComponent.SetSound` (`self.Audio`) `New Sound`)
  (`AudioComponent.Play` (`self.Audio`) 0.0))

(fn `Declare Game Over`
  (if (`|EnumEquality` (`self.Game State`) "NewEnumerator0")
    (`/Game/VGDC_VR/Blueprints/BPFL_DebugPrinting.Print Debug` "GameState is declaring Game Over!" true "NewEnumerator0" self)
    (set `self.Game State` "NewEnumerator2")
    (`self.Change Music` (`self.Music - Game Over`))
    (`/Game/VGDC_VR/Player/BP_VRPawn.On Game Over` (`self.Player Pawn`))
    (`/Game/VGDC_VR/Environment/Lighting/BP_SceneLighting.Fade Out` (`self.Scene Lighting`) 0)
    (else
      (`/Game/VGDC_VR/Blueprints/BPFL_DebugPrinting.Print Debug` (`KismetStringLibrary.Concat_StrStr` "GameState called to Delcare Game Over, but we aren't in play! Current play state: " (`|GetEnumeratorNameAsString` (`self.Game State`))) true "NewEnumerator1" self))))

(fn `Get Total Score`
  (returns (`Total Score` :type Integer))
  (return (`/Game/VGDC_VR/Core/BPFL_CoreUtilities.CalculateTotalScore` (`self.Level Stats`) (`/Game/VGDC_VR/Player/BP_VRPawn.Get Cumulative Weapon Stats` (`self.Player Pawn`)))))

(fn `Start Game`
  (`/Game/VGDC_VR/Blueprints/BPFL_DebugPrinting.Print Debug` "Game State is Starting Game!" true "NewEnumerator0" self)
  (set `self.Game State` "NewEnumerator0")
  (`self.Change Music` (`self.Music - Tunnel`)))

(fn `Start Hub Platform Transition`
  (set `self.Game State` "NewEnumerator5"))

(fn `Update Level Stats`
  (bind _tunnel_manager (`self.Tunnel Manager`))
  (`/Engine/EditorBlueprintResources/StandardMacros.IsValid` _tunnel_manager
    (:`Is Valid`
      (set `self.Level Stats` (make `/Game/VGDC_VR/Core/LevelStats` (`/Game/VGDC_VR/Environment/Technical/BP_TunnelManager.Current Level` _tunnel_manager) (`/Game/VGDC_VR/Environment/Technical/BP_TunnelManager.Get Current Speed Multiplier` _tunnel_manager))))
    (:`Is Not Valid`
      (`/Game/VGDC_VR/Blueprints/BPFL_DebugPrinting.Print Debug` "Game state tried to update stats, but tunnel manager is invalid!" true "NewEnumerator2" self))))

(fn `UserConstructionScript`)