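; PoolableObject_BP is an actor meant for object pooling that retires itself after a period of activity.
; Tick accumulates delta time in InactiveTimer and, once it reaches InactiveTime, resets the timer and calls Destroy.
; Despite its name, Destroy only disables tick and collision and hides the actor, leaving the instance alive; reactivation is not handled here.
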(event `self.ReceiveTick`
  (params (DeltaSeconds :type "Float (single-precision)"))
  (set `self.inactiveTimer` (+ DeltaSeconds (`self.inactiveTimer`)))
  (if (>= (`self.inactiveTimer`) (`self.inactiveTime`))
    (set `self.inactiveTimer` 0.0)
    (`self.Destroy`)))

(fn `Destroy`
  (`self.SetActorTickEnabled` false)
  (`self.SetActorHiddenInGame` true)
  (`self.SetActorEnableCollision` false))

(fn `UserConstructionScript`)