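; Object pool actor that recycles instances of a configurable Actor class to limit spawning.
; CreateActor reuses a hidden instance or spawns one while below MaxSize, then positions and activates it, passing itself to BPI_Poolable actors.
; Hidden state marks availability, with ActivityToggle also switching tick and collision.
; When Shrink is on, a Tick timer periodically destroys one inactive instance while the pool exceeds MinSize.
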(event `self.ReceiveBeginPlay`)

(event `self.ReceiveEndPlay`
  (params (EndPlayReason :type "EEndPlayReason Enum" :default "Destroyed"))
  (`self.shrinkPool`))

(event `self.ReceiveTick`
  (params (DeltaSeconds :type "Float (single-precision)"))
  (if (`self.shrink`)
    (bind _output_get (set `self.shrinkTimer` (+ DeltaSeconds (`self.shrinkTimer`))))
    (`/Game/VGDC_VR/Core/Utilities/BPFL_DebugPrinting.Print Debug` "Object pool will be shrinking! (Timer expired)" true "NewEnumerator4" self)
    (if (>= _output_get (`self.shrinkTime`))
      (set `self.shrinkTimer` 0.0)
      (if (> (`self.currentPoolSize`) (`self.minSize`))
        (`/Game/VGDC_VR/Core/Utilities/BPFL_DebugPrinting.Print Debug` "Object pool has enough elements to shrink!" true "NewEnumerator4" self)
        (`self.shrinkPool`)
        (else
          (`/Game/VGDC_VR/Core/Utilities/BPFL_DebugPrinting.Print Debug` "Object pool does not have enough elements to shrink!" true "NewEnumerator4" self))))))

(fn `activityToggle`
  (params (obj :type "Actor Object Reference") (active :type Boolean))
  (locals (hideToggle :type Boolean :default false) (collisionToggle :type Boolean :default true) (tickerToggle :type Boolean :default true))
  (bind _active (`local.active`))
  (`/Engine/EditorBlueprintResources/StandardMacros.IsValid` obj
    (:`Is Valid`
      (`/Game/VGDC_VR/Core/Utilities/BPFL_DebugPrinting.Print Debug` (`KismetStringLibrary.Concat_StrStr` "Toggling actor activity: " (`KismetSystemLibrary.GetDisplayName` obj) "'s activity is now " (`KismetStringLibrary.Conv_BoolToString` active)) (`self.Print Debug Messages`) "NewEnumerator4" self)
      ;[0.4423 1 0.4684] Active = not hidden
      (`self.SetActorHiddenInGame` obj (not active))
      ;[0.8818 0.5831 1] Active = tickable and collidable
      (`self.SetActorTickEnabled` obj _active)
      (`self.SetActorEnableCollision` obj _active))
    (:`Is Not Valid`
      (`/Game/VGDC_VR/Core/Utilities/BPFL_DebugPrinting.Print Debug` "Object pooler called Activity Toggle on null element!" true "NewEnumerator2" self))))

(fn `anyObjectsInactive`
  (returns (anyInactive :type Boolean))
  (locals (inactive :type Boolean))
  (bind _objpool (`self.objPool`))
  (for _index (range (`KismetArrayLibrary.Array_Length` _objpool))
    (if (`Actor.bHidden` (`|GetArrayItem` _objpool _index))
      (bind _output_get (set `local.inactive` true))
      (return _output_get)))
  (return _output_get))

(fn `createActor`
  (params (position :type "Vector Structure") (rotation :type "Rotator Structure"))
  (returns (pooledObj :type "Actor Object Reference"))
  (locals (anyInactive :type Boolean) (count :type Integer) (obj :type "Actor Object Reference"))
  (bind _obj (`local.obj`))
  (bind _objpool (`self.objPool`))
  (bind _output (`|GetArrayItem` (`self.objPool`) (`local.count`)))
  ;[0.8646 0.709 0] Are there any inactive objects in the pool?
  (if (`self.anyObjectsInactive`)
    (set `local.count` 0)
    ;[0.009825 0.9583 0.1795] Search for the first inactive instance within the pool and set reference to it
    (while (and (== (`local.obj`) null) (< (`local.count`) (`KismetArrayLibrary.Array_Length` (`self.objPool`))))
      (if (`Actor.bHidden` _output)
        (set `local.obj` _output))
      (`/Engine/EditorBlueprintResources/StandardMacros.IncrementInt` (`local.count`)))
    (`/Game/VGDC_VR/Core/Utilities/BPFL_DebugPrinting.Print Debug` (`KismetStringLibrary.Concat_StrStr` "Pooler.createActor will use the inactive actor: " (`KismetSystemLibrary.GetDisplayName` (`local.obj`))) (`self.Print Debug Messages`) "NewEnumerator4" self)
    (else
      ;[0.08778 1 0.9003] If not, is the current pool size less than its maximum capacity? (maxSize)
      (if (< (`self.currentPoolSize`) (`self.maxSize`))
        ;[0 0.01656 0.3125] Spawn a new instance if there are no objects in the pool that are inactive
        (bind _returnvalue (`|SpawnActorFromClass` (`self.poolObj`) (`self.GetTransform`) "Undefined" "OverrideRootScale" null null))
        (set `local.obj` _returnvalue)
        ;[1 0 0.2166] Add new instance to the pool and update pool size variable
        (`KismetArrayLibrary.Array_Add` _objpool (`local.obj`))
        (set `self.currentPoolSize` (`KismetArrayLibrary.Array_Length` _objpool))
        (`/Game/VGDC_VR/Core/Utilities/BPFL_DebugPrinting.Print Debug` (`KismetStringLibrary.Concat_StrStr` "Pooler.createActor just created a " "new poolable, as none were available: " (`KismetSystemLibrary.GetDisplayName` (`local.obj`))) (`self.Print Debug Messages`) "NewEnumerator4" self)
        (else
          (`/Game/VGDC_VR/Core/Utilities/BPFL_DebugPrinting.Print Debug` (`KismetStringLibrary.Concat_StrStr` "Pool has already reached limit! " (`KismetStringLibrary.Concat_StrStr` (`/Game/VGDC_VR/Core/Utilities/BPFL_DebugPrinting.Debug Format Int` "Current Size" (`self.currentPoolSize`)) ">" (`/Game/VGDC_VR/Core/Utilities/BPFL_DebugPrinting.Debug Format Int` "Max Size" (`self.maxSize`)))) (`self.Print Debug Messages`) "NewEnumerator1" self)
          (return null)))))
  ;[0.1812 0.4989 1] Prepare actor and return
  (`self.K2_SetActorLocationAndRotation` (`local.obj`) (`local.position`) (`local.rotation`) false false)
  (`self.activityToggle` (`local.obj`) true)
  (if (`KismetSystemLibrary.DoesImplementInterface` _obj "/Game/VGDC_VR/Core/Pooling/BPI_Poolable.BPI_Poolable_C")
    (message `/Game/VGDC_VR/Core/Pooling/BPI_Poolable.Set Pool` _obj self))
  (return _obj))

(fn `createPool`
  ;[1 0 0] Creates a pool of Actors, with the count being equal the mininum pool size (minSize)
  (`/Game/VGDC_VR/Core/Utilities/BPFL_DebugPrinting.Print Debug` (`KismetStringLibrary.Concat_StrStr` "Object pool is creating " (`/Game/VGDC_VR/Core/Utilities/BPFL_DebugPrinting.Debug Format Int` "" (`self.minSize`)) " actors!") true "NewEnumerator4" self)
  (for _ (range (+ (`self.minSize`) 1))
    (`self.createActor` (`self.spawnPos`))))

(fn `deleteActor`
  (params (object :type "Actor Object Reference"))
  (bind _objpool (`self.objPool`))
  ;[1 0 0] Removes actor from object pool, destroys it, and proceeds to update pool size variable (currentPoolSize)
  (`KismetArrayLibrary.Array_RemoveItem` _objpool object)
  (`self.K2_DestroyActor` object)
  (set `self.currentPoolSize` (`KismetArrayLibrary.Array_Length` _objpool)))

(fn `findFirstInactive`
  (returns (object :type "Actor Object Reference"))
  ;[0.8646 0.709 0] Returns the first inactive instance in the object pool
  (`KismetSystemLibrary.PrintString` "Hello")
  (for _array_element (`self.objPool`)
    (if (`Actor.bHidden` _array_element)
      (return _array_element)))
  (return null) ; No object found; return null
)

(fn `hidePool`
  (for _array_element (`self.objPool`)
    (`self.activityToggle` _array_element)))

(fn `setPooledObject`
  (params (pooledObj :type "Actor Class Reference")))

(fn `shrinkPool`
  ;[0 0.01656 0.3125] Checks if any objects are inactive within the pool, and deletes the first instance
  (if (`self.anyObjectsInactive`)
    (`self.deleteActor` (`self.findFirstInactive`))))

(fn `UserConstructionScript`)