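; Score-keeping Blueprint for the VR game that loads a leaderboard from a filename on BeginPlay.
; Loading and adding high scores rely on functions defined outside this graph, and the game-over event is an empty stub.
; Debug helpers print all scores or add random fake scores within configurable bounds, with editor functions for preset batch sizes.
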(event `self.ReceiveBeginPlay`
  (`self.LoadLeaderboard` (`self.Filename`)))

(event `OnGameOver`)

(fn `[Editor] Add 1 Fake Score`
  (`self.Add Fake Scores` 1))

(fn `[Editor] Add 10 Fake Scores`
  (`self.Add Fake Scores` 10))

(fn `[Editor] Add 100 Fake Scores`
  (`self.Add Fake Scores` 100))

(fn `Add Fake Scores`
  (params (Count :type Integer :default 10))
  (locals (defaultNames :type "Array of String") (scores :type "Map of String to Object Object Reference") (`High Scores` :type "Array of ScoreContainer Object Reference"))
  (bind (_x _y) (`KismetMathLibrary.BreakVector2D` (`self.Fake Score Bounds`)))
  (for _ (range 1 (+ Count 1))
    (`self.AddHighScoreContainer` (`ScoreContainer.CreateRandomScoreContainer` 3 3 (`KismetMathLibrary.FTrunc` _x) (`KismetMathLibrary.FTrunc` _y)))))

(fn `PrintAllScores`
  (params (HighScores :type "Array of ScoreContainer Object Reference"))
  (for _index (range (`KismetArrayLibrary.Array_Length` HighScores))
    (`KismetSystemLibrary.PrintString` (`ScoreContainer.ToString` (`|GetArrayItem` (`local.HighScores`) _index)))))

(fn `UserConstructionScript`)