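; BP_Projectile is a projectile actor that flies straight along its forward vector until it hits something or expires.
; Each Tick adds delta time to Lifetime, then either destroys the actor at MaxLifetime or offsets it by Velocity scaled by delta time.
; Movement is a manual world offset without sweep.
; A Hit event destroys the projectile unless the other actor's class is VRPawn.
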(event `self.ReceiveHit`
  (params (MyComp :type "PrimitiveComponent Object Reference") (Other :type "Actor Object Reference") (OtherComp :type "PrimitiveComponent Object Reference") (bSelfMoved :type Boolean) (HitLocation :type "Vector Structure") (HitNormal :type "Vector Structure") (NormalImpulse :type "Vector Structure") (Hit :type "HitResult Structure (by ref)"))
  ;[1 0.4939 0.333] Destroy on collision
  (if (!= (`GameplayStatics.GetObjectClass` Other) "/Script/VGDC_VR.VRPawn")
    (`self.K2_DestroyActor`)))

(event `self.ReceiveTick`
  (params (DeltaSeconds :type "Float (single-precision)"))
  ;[0.2317 0.3675 1] Increment Lifetime
  (bind _output_get (set `self.Lifetime` (+ DeltaSeconds (`self.Lifetime`))))
  ;[0.9371 0.4447 1] Check if expired
  (if (>= _output_get (`self.MaxLifetime`))
    (`self.K2_DestroyActor`)
    (else
      ;[0.2912 1 0.2907] Move across world
      (`self.K2_AddActorWorldOffset` (* (`self.GetActorForwardVector`) (* DeltaSeconds (`self.Velocity`)))))))

(fn `UserConstructionScript`)