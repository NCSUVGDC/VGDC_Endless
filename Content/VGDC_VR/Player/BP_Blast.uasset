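; BP_Blast is a projectile actor that destroys doors it hits.
; Each tick it moves along its forward vector at a set velocity without sweeping, and destroys itself once its lifetime runs out.
; When its BlastCollision overlaps a BP_Door of that exact class with hit points left, it calls DestroyDoor on it and then destroys itself.
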(event `self.BlastCollision.OnComponentBeginOverlap`
  (params (OverlappedComponent :type "PrimitiveComponent Object Reference") (OtherActor :type "Actor Object Reference") (OtherComp :type "PrimitiveComponent Object Reference") (OtherBodyIndex :type Integer) (bFromSweep :type Boolean) (SweepResult :type "HitResult Structure (by ref)"))
  ;[1 1 1] If it hits a closed door, destroy that door
  (bind _asbp_door (cast `/Game/VGDC_VR/Environment/Door/BP_Door` OtherActor))
  (if (and (> (`/Game/VGDC_VR/Environment/Door/BP_Door.Door Hit Points` _asbp_door) 0) (== (`GameplayStatics.GetObjectClass` OtherActor) "/Game/VGDC_VR/Environment/Door/BP_Door.BP_Door_C"))
    (`/Game/VGDC_VR/Environment/Door/BP_Door.Destroy Door` _asbp_door)
    (`self.K2_DestroyActor`)))

(event `self.ReceiveTick`
  (params (DeltaSeconds :type "Float (single-precision)"))
  ;[0.2317 0.3675 1] Increment Lifetime
  (bind _output_get (set `self.Lifetime` (+ DeltaSeconds (`self.Lifetime`))))
  ;[0.9371 0.4447 1] Check if expired
  (if (>= _output_get (`self.MaxLifetime`))
    (`self.K2_DestroyActor`)
    (else
      ;[0.2912 1 0.2907] Move across world
      (`self.K2_AddActorWorldOffset` (* (`self.GetActorForwardVector`) (* DeltaSeconds (`self.Velocity`)))))))

(fn `UserConstructionScript`)