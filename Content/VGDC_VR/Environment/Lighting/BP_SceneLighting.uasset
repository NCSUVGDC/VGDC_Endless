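; BP_SceneLighting controls a scene's ambient lighting through post process settings and fades it out and back in.
; A Fade timeline scales ambient intensity, dims cells via a global material parameter collection on a fourth-power curve, and optionally changes saturation.
; FadeIn plays the same timeline in reverse.
; The construction script derives play rate from FadeTime and sets initial tint and intensity, or zero intensity when off by default.
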(event `/Game/VGDC_VR/Core/BPI_NeedsGameState.Set BP_BaseGameState`
  (params (State :type "/Game/VGDC_VR/Core/BP_BaseGameState Object Reference"))
  (set `self.GameState` State))

(event `Fade Out`
  (params (`Affects Saturation` :type Boolean :default true))
  (set `self.Should Affect Saturation` `Affects Saturation`)
  (bind (_direction _brightness _saturation) (`Timeline|Fade` :!via `PlayFromStart` :!label _label)
    (:`Update`
      (`|ExecutionSequence`
        (:`then_0`
          ;[1 1 1] Change Lighting
          (setmembers `PostProcessSettings` :`StructRef` (`PostProcessComponent.Settings` (`self.Ambient Lighting`)) :`AmbientCubemapIntensity` (* (`self.Default Lighting Intensity`) _brightness))
          (`KismetMaterialLibrary.SetScalarParameterValue` "/Game/VGDC_VR/Materials/M_GlobalLightDimming.M_GlobalLightDimming" "Brightness" (`KismetMathLibrary.MultiplyMultiply_FloatFloat` _brightness 4.0)) ; Dim Cells
        )
        (:`then_1`
          ;[1 1 1] Optionally affect saturation
          (if (`self.Should Affect Saturation`)
            (setmembers `PostProcessSettings` :`StructRef` (`PostProcessComponent.Settings` (`self.Ambient Lighting`)) :`ColorSaturation` (`KismetMathLibrary.MakeVector4` _saturation _saturation _saturation _saturation))))))))

(event `Fade In`
  (params (`Affect Saturation` :type Boolean))
  (set `self.Should Affect Saturation` `Affect Saturation`)
  (goto _label :!via `ReverseFromEnd`))

(fn `Fade Effect`)

(fn `UserConstructionScript`
  ;[1 1 1] Update Fade In/Fade Out Play Rate
  (`TimelineComponent.SetPlayRate` (`self.Fade`) (/ 1.0 (`self.Fade Time`)))
  (if (`self.On By Default`)
    ;[1 1 1] Updating Ambient Lighting Intensity
    (setmembers `PostProcessSettings` :`StructRef` (`PostProcessComponent.Settings` (`self.Ambient Lighting`)) :`AmbientCubemapTint` (`self.Default Lighting Tint`) :`AmbientCubemapIntensity` (`self.Default Lighting Intensity`))
    (else
      ;[1 1 1] Disable lighting if not enabled
      (setmembers `PostProcessSettings` :`StructRef` (`PostProcessComponent.Settings` (`self.Ambient Lighting`)) :`AmbientCubemapIntensity` 0.0))))