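; BP_Door is a VR door actor that procedurally covers itself in crystal components totalling a target hit-point value.
; Tick polls an editor-set flag to run GenerateCrystals, then prints the following frame's delta time as generation cost.
; Generation clears old crystals, then adds random difficulties from a hit-point-to-color map, capped near the remaining health, until CurrentHealth reaches the target.
; Each crystal gets a random relative location and a tinted dynamic material.
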(event `self.ReceiveBeginPlay`)

(event `self.ReceiveTick`
  (params (DeltaSeconds :type "Float (single-precision)"))
  ;[1 1 1] Log the last frame's deltaTime after generating crystals
  (if (`self.Get Next DT`)
    (set `self.Get Next DT` false)
    (`KismetSystemLibrary.PrintString` (`KismetStringLibrary.Concat_StrStr` "Took " (`KismetStringLibrary.Conv_DoubleToString` DeltaSeconds) " seconds to generate " (`KismetStringLibrary.Conv_IntToString` (`KismetArrayLibrary.Array_Length` (`self.Crystals`))) " door crystals") true true (struct :`R` 1.0 :`G` 0.975386 :`A` 1.0) 5.0))
  ;[1 1 1] Generate Crystals when the button is clicked in the editor
  (if (`self.Editor Generate Crystals `)
    (set `self.Editor Generate Crystals ` false)
    (`self.Generate Crystals` (`self.Door Hit Points`))
    (set `self.Get Next DT` true)))

(fn `Add Crystal`
  (params (`Initial HP` :type Integer :default 1) (Color :type "LinearColor Structure"))
  (returns (`New Crystal` :type "CrystalComponent Object Reference"))
  (bind _returnvalue (`AddComponent|NODE_AddCrystalComponent-2` :`RelativeTransform` (`KismetMathLibrary.MakeTransform` (`KismetMathLibrary.MakeVector` (* (`KismetMathLibrary.RandomFloatInRange` -2.0 2.0) 100.0) (* (`KismetMathLibrary.RandomFloatInRange` -2.0 2.0) 100.0) (* (`KismetMathLibrary.RandomFloatInRange` -2.0 2.0) 100.0))) :`HitPoints` `Initial HP`))
  ;[0.3133 0.8901 1] Set Mesh
  (`StaticMeshComponent.SetStaticMesh` (`CrystalComponent.CrystalMesh` _returnvalue) (`self.Crystal Mesh`))
  ;[0.2395 0.3166 1] Create dynamic material
  (bind _returnvalue_2 (`KismetMaterialLibrary.CreateDynamicMaterialInstance` (`self.Master Crystal Material`)))
  (`MaterialInstanceDynamic.SetVectorParameterValue` _returnvalue_2 "Color" (`local.Color`))
  ;[0.7498 0.07785 1] Assign new material
  (`PrimitiveComponent.SetMaterial` (`CrystalComponent.CrystalMesh` _returnvalue) 0 _returnvalue_2)
  ;[1 0 0.06674] Add crystal to array
  (`KismetArrayLibrary.Array_Add` (`self.Crystals`) _returnvalue)
  (return _returnvalue))

(fn `Choose New Crystal Difficulty`
  (params (`Max Hit Points` :type Integer :default 11))
  (returns (`Hit Points` :type Integer) (Color :type "LinearColor Structure"))
  (locals (`Max Difficulty Index` :type Integer :default -1) (`New Hit Points` :type Integer))
  (bind _crystal_difficulties (`self.Crystal Difficulties`))
  (if (> `Max Hit Points` 0)
    ;[0.1129 0.7683 1] Find what the index of the highest difficulty level we can choose from without going over the Max Hit Points constraint
    (bind _keys (`BlueprintMapLibrary.Map_Keys` (`self.Crystal Difficulties`)))
    ;;[1 1 1] Default Index = Highest
    (set `local.Max Difficulty Index` (- (`KismetArrayLibrary.Array_Length` _keys) 1))
    (for (_array_element _array_index) _keys
      (if (>= _array_element (`local.Max Hit Points`))
        (set `local.Max Difficulty Index` _array_index)
        (break)))
    ;[0.2891 0.3467 1] Randomly select the difficulty level and color within our max difficulty constraint
    (bind _keys_2 (`BlueprintMapLibrary.Map_Keys` _crystal_difficulties))
    (bind _output_get (set `local.New Hit Points` (`|GetArrayItem` _keys_2 (`KismetMathLibrary.RandomIntegerInRange` 0 (`local.Max Difficulty Index`))))) ; Must be set as variable, or we'll accidentally use the RNG twice
    (return _output_get (`BlueprintMapLibrary.Map_Find` _crystal_difficulties _output_get))
    (else
      ;[1 0.1615 0.1615] Function should quit if given an invalid Max Hit Points
      (`KismetSystemLibrary.PrintString` "Invalid New Crystal Difficulty!" true true (struct :`R` 1.0 :`A` 1.0))
      (return -1))))

(fn `Generate Crystals`
  (params (`Door Health` :type Integer :default 6))
  (locals (CurrentHealth :type Integer :default 0) (MaxCrystalHealth :type Integer))
  ;[1 1 1] Remove old crystals
  (for _array_element (`self.Crystals`)
    (`ActorComponent.K2_DestroyComponent` _array_element))
  (`KismetArrayLibrary.Array_Clear` (`self.Crystals`))
  ;[1 1 1] Generate crystals until we reach Door Health
  (while (> `Door Health` (`local.CurrentHealth`))
    ;;[0.3904 0.797 1] Choose Crystal Parameters
    (bind (_hit_points _color) (`self.Choose New Crystal Difficulty` (- (`local.Door Health`) (`local.CurrentHealth`))))
    ;;[0.277 0.3519 1] Add Crystal
    (bind _new_crystal (`self.Add Crystal` _hit_points _color))
    ;;[1 1 1] Increment Current Health
    (set `local.CurrentHealth` (+ (`local.CurrentHealth`) (`CrystalComponent.HitPoints` _new_crystal)))))

(fn `UserConstructionScript`)