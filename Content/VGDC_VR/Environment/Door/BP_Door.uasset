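; VR door that covers its mesh with pooled crystals whose combined hit points aim to match the door's health.
; InitializeDoor releases old crystals, then pulls new ones from the BP_CrystalPooler singleton and snaps them to random or sequential mesh sockets.
; Generation stops at target health, when sockets run out, or via a loop-count killswitch.
; Tick polls a boolean acting as an editor generate button and handles timing logs and debug drawing.
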(event `self.ReceiveBeginPlay`
  ;[1 0.7334 0.3291] Make sure we have a pool!
  (bind _pooler (`/Game/VGDC_VR/Environment/Pooling/BP_PoolerHelperMacros.Get Pooler Singleton` "/Game/VGDC_VR/Environment/Pooling/BP_CrystalPooler.BP_CrystalPooler_C")
    (:`Exec Out`
      (bind _asbp_crystal_pooler (cast `/Game/VGDC_VR/Environment/Pooling/BP_CrystalPooler` _pooler))
      (set `self.Crystal Pool` _asbp_crystal_pooler))))

(event `self.ReceiveTick`
  (params (DeltaSeconds :type "Float (single-precision)"))
  (bind _doormesh (`self.DoorMesh`))
  (`|ExecutionSequence`
    (:`then_0`
      ;[0 1 0.1319] Generate Crystals when the button is clicked in the editor
      (if (`self.Editor Generate Crystals `)
        (set `self.Editor Generate Crystals ` false)
        (`self.Initialize Door` (`self.Door Hit Points`))))
    (:`then_1`
      ;[1 0.8989 0] Log the last frame's deltaTime after generating crystals
      (if (`self.Debug Crystal Gen Time`)
        (set `self.Debug Crystal Gen Time` false)
        (`/Game/VGDC_VR/Blueprints/BPFL_DebugPrinting.Print Debug` (`KismetStringLibrary.Concat_StrStr` "Took " (`KismetStringLibrary.Conv_DoubleToString` DeltaSeconds) " seconds to generate " (`KismetStringLibrary.Conv_IntToString` (`KismetArrayLibrary.Array_Length` (`self.Crystals`))) " door crystals") true "NewEnumerator1" self)))
    (:`then_2`
      ;[0 0 0] Debug Drawing
      (if (`self.Debug Draw Stuff`)
        (`|ExecutionSequence`
          (:`then_0`
            (for _array_element (`self.Crystals`)
              (`KismetSystemLibrary.DrawDebugSphere` (`self.K2_GetActorLocation` _array_element) 100.0 8 (struct :`R` 1.0 :`G` 0.008842 :`A` 1.0) 0.0 1.0)))
          (:`then_1`
            (for _array_element_2 (`SceneComponent.GetAllSocketNames` _doormesh)
              (`KismetSystemLibrary.DrawDebugBox` (.location (`SceneComponent.GetSocketTransform` _doormesh _array_element_2 "RTS_World")) (50.0 50.0 50.0) (struct :`R` 0.599752 :`G` 0.239298 :`B` 1.0 :`A` 1.0) (.rotation (`SceneComponent.GetSocketTransform` _doormesh _array_element_2 "RTS_World")) 0.0 2.0)))
          (:`then_2`
            (for _array_element_3 (`SceneComponent.GetAllSocketNames` (`self.DoorMesh`))
              (bind (_value _returnvalue) (`BlueprintMapLibrary.Map_Find` (`self.OccupiedSockets`) _array_element_3))
              (if _returnvalue
                (bind _location (.location (`SceneComponent.GetSocketTransform` (`self.DoorMesh`) _array_element_3 "RTS_World")))
                (`KismetSystemLibrary.DrawDebugBox` _location (40.0 40.0 40.0) (struct :`R` 0.104591 :`G` 0.563506 :`B` 1.0 :`A` 1.0) (.rotation (`SceneComponent.GetSocketTransform` (`self.DoorMesh`) _array_element_3 "RTS_World")) 0.0 2.0)
                (`KismetSystemLibrary.DrawDebugString` _location (`KismetStringLibrary.Concat_StrStr` (`KismetSystemLibrary.GetDisplayName` _value)) null (struct :`R` 1.0 :`B` 0.043376 :`A` 1.0)) ; Every day I start to hate this game engine more an more. this just doesn't work.
              ))))))))

(fn `Add Crystal`
  (params (`Min Hitpoints` :type Integer :default 1) (`Max Hitpoints` :type Integer :default 5))
  (returns (`New Crystal` :type "/Game/VGDC_VR/Environment/PowerCell/BP_Crystal Object Reference"))
  ;[1 1 1] Pull Crystal from Pooler and Initialize HP
  (bind _pooledobj (`/Game/VGDC_VR/Environment/Pooling/ObjectPooler_BP.createActor` :`self` (`self.Crystal Pool`)))
  (bind _asbp_crystal (cast `/Game/VGDC_VR/Environment/PowerCell/BP_Crystal` _pooledobj))
  (bind _crystal (`/Game/VGDC_VR/Environment/PowerCell/BP_Crystal.Initialize Crystal` _asbp_crystal (`local.Min Hitpoints`) (`local.Max Hitpoints`) self))
  (`KismetArrayLibrary.Array_Add` (`self.Crystals`) _crystal)
  ;[1 1 1] Put Crystal on a Socket
  (bind _successful (`self.Attach Crystal To Door` _crystal))
  (if _successful
    (return _crystal)
    (else
      (`/Game/VGDC_VR/Blueprints/BPFL_DebugPrinting.Print Debug` "Ran out of room for crystals! No more sockets available! " true "NewEnumerator2" self)
      (return null))))

(fn `Attach Crystal To Door`
  (params (Crystal :type "/Game/VGDC_VR/Environment/PowerCell/BP_Crystal Object Reference"))
  (returns (Successful :type Boolean))
  (locals (`Chosen Socket` :type Name))
  ;[1 1 1] Make sure sockets are available
  (if (> (`KismetArrayLibrary.Array_Length` (`self.Available Sockets`)) 0)
    (if (`self.Random Socket Selection`)
      ;[1 0.396 0.9766] Choose Socket Randomly
      (set `local.Chosen Socket` (`|GetArrayItem` (`self.Available Sockets`) (`KismetMathLibrary.RandomIntegerInRange` 0 (- (`KismetArrayLibrary.Array_Length` (`self.Available Sockets`)) 1))))
      (else
        ;[0.4461 0.4314 1] Get Next Available Socket
        (set `local.Chosen Socket` (`|GetArrayItem` (`self.Available Sockets`)))))
    ;[0.5068 0.3773 1] Socket found, attach the mesh and exit
    (`KismetArrayLibrary.Array_RemoveItem` (`self.Available Sockets`) (`local.Chosen Socket`))
    (`BlueprintMapLibrary.Map_Add` (`self.OccupiedSockets`) (`local.Chosen Socket`) (`local.Crystal`))
    (`self.K2_AttachToComponent` (`local.Crystal`) (`self.DoorMesh`) (`local.Chosen Socket`) "SnapToTarget" "SnapToTarget" "SnapToTarget" true)
    (if (== (`SceneComponent.GetSocketLocation` (`self.DoorMesh`) (`local.Chosen Socket`)) (`self.K2_GetActorLocation` (`local.Crystal`)) :`ErrorTolerance` 0.01)
      (`/Game/VGDC_VR/Blueprints/BPFL_DebugPrinting.Print Debug` (`KismetStringLibrary.Concat_StrStr` "Crystal " (`KismetSystemLibrary.GetDisplayName` (`local.Crystal`)) " successfully attached to socket " (`KismetStringLibrary.Conv_NameToString` (`local.Chosen Socket`))) true "NewEnumerator4" self)
      (else
        (`/Game/VGDC_VR/Blueprints/BPFL_DebugPrinting.Print Debug` (`KismetStringLibrary.Concat_StrStr` "Crystal " (`KismetSystemLibrary.GetDisplayName` (`local.Crystal`)) " unsuccessfully attached to socket " (`KismetStringLibrary.Conv_NameToString` (`local.Chosen Socket`))) true "NewEnumerator2" self)
        (`/Game/VGDC_VR/Blueprints/BPFL_DebugPrinting.Print Debug` (`KismetStringLibrary.Concat_StrStr` "Crystal location: " (`KismetStringLibrary.Conv_VectorToString` (`self.K2_GetActorLocation` (`local.Crystal`))) " Socket Location:" (`KismetStringLibrary.Conv_VectorToString` (`SceneComponent.GetSocketLocation` (`self.DoorMesh`) (`local.Chosen Socket`)))) true "NewEnumerator2" self)))
    (return true)
    (else
      ;[1 0.4694 0.2159] No socket found for crystal n
      (`self.K2_SetActorLocation` (`local.Crystal`) (+ (`self.K2_GetActorLocation`) (* (50.0 0.0 0.0) (`KismetArrayLibrary.Array_Length` (`self.Crystals`)))) false false)
      (return false))))

(fn `Initialize Door`
  (params (`Door Health` :type Integer :default 6))
  (locals (CurrentHealth :type Integer :default 0) (`Selected Max Crystal Health` :type Integer) (WhileLoopCounter :type Integer) (QuitPrematurely :type Boolean))
  (bind _max_crystal_hp (`self.Max Crystal HP`))
  (bind _returnvalue (- (`local.Door Health`) (`local.CurrentHealth`)))
  (set `self.Door Hit Points` `Door Health`)
  (`self.Release Crystals`)
  ;[1 0.3848 0.675] Reset sockets
  (set `self.Available Sockets` (`SceneComponent.GetAllSocketNames` (`self.DoorMesh`)))
  (`BlueprintMapLibrary.Map_Clear` (`self.OccupiedSockets`))
  ;[0.295 1 0.05254] Generate crystals until we reach Door Health
  (while (and (> (`local.Door Health`) (`local.CurrentHealth`)) (not (`local.QuitPrematurely`)))
    (bind _result (`/Engine/EditorBlueprintResources/StandardMacros.IncrementInt` (`local.WhileLoopCounter`))
      (:`  `
        (if (>= _result 100)
          (set `local.CurrentHealth` (`local.Door Health`))
          (`/Game/VGDC_VR/Blueprints/BPFL_DebugPrinting.Print Debug` "INFINITE LOOP KILLSWITCH ENGAGED" true "NewEnumerator2" self))
        ;;[0.3904 0.797 1] Choose Crystal HP Parameters
        (if (> _max_crystal_hp 0)
          (set `local.Selected Max Crystal Health` (`KismetMathLibrary.Min` _max_crystal_hp _returnvalue)) ; If max health is specified, choose lesser of current health and max HP
          (else
            (set `local.Selected Max Crystal Health` _returnvalue) ; If max health is not specified, use health remaining
          ))
        ;;[0.277 0.3519 1] Add Crystal
        (bind _new_crystal (`self.Add Crystal` (`KismetMathLibrary.Clamp` (`self.Min Crystal HP`) 0 (`local.Selected Max Crystal Health`)) (`local.Selected Max Crystal Health`)))
        (`/Engine/EditorBlueprintResources/StandardMacros.IsValid` _new_crystal
          (:`Is Valid`
            ;;[1 0.4172 0.6975] Increment Current Health
            (set `local.CurrentHealth` (+ (`local.CurrentHealth`) (`/Game/VGDC_VR/Environment/PowerCell/BP_Crystal.Hit Points` _new_crystal))))
          (:`Is Not Valid`
            ;[1 0.01661 0] Stop generating if the door ran out of room
            (`/Game/VGDC_VR/Blueprints/BPFL_DebugPrinting.Print Debug` (`KismetStringLibrary.Concat_StrStr` "Crystal generation stopped prematurely! " "Final Hitpoints: " (`KismetStringLibrary.Conv_IntToString` (`local.CurrentHealth`))) true "NewEnumerator2" self)
            (set `local.QuitPrematurely` true))))))
  (set `self.Debug Crystal Gen Time` true))

(fn `Release Crystals`
  (for _array_element (`self.Crystals`)
    (`self.K2_DetachFromActor` _array_element "KeepRelative" "KeepRelative" "KeepRelative")
    (`/Game/VGDC_VR/Environment/Pooling/ObjectPooler_BP.activityToggle` (`self.Crystal Pool`) _array_element false))
  (`KismetArrayLibrary.Array_Clear` (`self.Crystals`)))

(fn `UserConstructionScript`)