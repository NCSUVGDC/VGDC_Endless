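; Shootable crystal target on a door, which loses hit points when shot during play and stays in place when destroyed.
; InitializeCrystal links the owning door and rolls starting hit points from difficulty keys within a min/max range.
; Damage notifies the door, spawns hit or destruction feedback, and recolors a dynamic material by health, dimming it to black at zero.
; An object pool reference is stored, but pooling on death is disabled.
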(event `/Game/VGDC_VR/Environment/Technical/BPI_Poolable.Set Pool`
  (params (Pool :type "/Game/VGDC_VR/Environment/Technical/ObjectPooler_BP Object Reference"))
  (set `self.Object Pool` Pool))

(fn `[EDITOR] Kill`
  (`self.Take Damage` (`self.Hit Points`)))

(fn `[EDITOR] Take Damage`
  (`ShootableInterface.OnShot`))

(fn `Choose Difficulty`
  (params (`Min Hit Points` :type Integer) (`Max Hit Points` :type Integer))
  (locals (`Max Index` :type Integer :default -1) (`Min Index` :type Integer :default -1))
  ;[1 1 1] Make sure our parameters are valid
  (if (and (<= `Min Hit Points` `Max Hit Points`) (> `Max Hit Points` 0))
    ;[0.1129 0.7683 1] Find what the index of the highest difficulty level we can choose from without going over the Max Hit Points constraint
    (bind _keys (`BlueprintMapLibrary.Map_Keys` (`self.Difficulty Colors DEPRECATED`)))
    ;;[1 1 1] Set Default Max Index
    (set `local.Max Index` (- (`KismetArrayLibrary.Array_Length` _keys) 1))
    ;;[0.776 0.726 0.137] Find the min/max indices
    (for (_array_element _array_index) _keys
      (`|ExecutionSequence`
        (:`then_0`
          ;;;[1 0.08323 0] Set max difficulty index
          (if (>= (`local.Max Hit Points`) _array_element)
            (set `local.Max Index` _array_index)))
        (:`then_1`
          ;;;[0.199 1 0] Set min difficulty index
          ;;;;[1 1 1] Only set the min difficulty once!
          (if (< (`local.Min Index`) 0)
            (if (<= (`local.Min Hit Points`) _array_element)
              (set `local.Min Index` _array_index))))))
    ;[0.7746 1 0.2891] Make sure min difficulty is set (e.g. if min hp = 0, it will not have been set)
    (set `local.Min Index` (`KismetMathLibrary.Clamp` (`local.Min Index`) 0 (`local.Max Index`)))
    ;[0.2891 0.3467 1] Randomly select the difficulty level within our max difficulty constraint
    (bind _keys_2 (`BlueprintMapLibrary.Map_Keys` (`self.Difficulty Colors DEPRECATED`)))
    (bind _output_get (set `self.Initial Hit Points` (`|GetArrayItem` _keys_2 (`KismetMathLibrary.RandomIntegerInRange` (`local.Min Index`) (`local.Max Index`)))))
    (set `self.Hit Points` _output_get)
    ;[0.898 0.3075 1] Set color
    (`self.Update Material`)
    (else
      ;;[1 0 0] Error message if parameters are invalid
      (`/Game/VGDC_VR/Blueprints/BPFL_DebugPrinting.Print Debug` (`/Game/VGDC_VR/Blueprints/BPFL_DebugPrinting.Debug Format Int Range` "Invalid New Crystal Difficulty" (`local.Min Hit Points`) (`local.Max Hit Points`)) true "NewEnumerator2" self)
      (return))))

(fn `Handle Destroyed Feedback`
  (`GameplayStatics.SpawnEmitterAttached` (`self.Destroyed Feedback Particle`) (`self.Mesh`) "None" (`self.Feedback Offset`))
  (`GameplayStatics.SpawnSoundAttached` (`self.Sound Destroyed`) (`self.Mesh`)))

(fn `Handle Hit Feedback`
  (`GameplayStatics.SpawnEmitterAttached` (`self.Hit Feedback Particle`) (`self.Mesh`) "None" (`self.Feedback Offset`)))

(fn `Initialize Crystal`
  (params (`Min Hitpoints` :type Integer) (`Max Hitpoints` :type Integer) (`Owning Door` :type "/Game/VGDC_VR/Environment/Door/BP_Door Object Reference"))
  (returns (Crystal :type "/Game/VGDC_VR/Environment/PowerCell/BP_Crystal Object Reference"))
  (`self.Choose Difficulty` `Min Hitpoints` `Max Hitpoints`)
  (set `self.Owning Door` `Owning Door`)
  (return self))

(fn `On Killed`
  (`self.Update Material`) ; Material is updated on shot, but update here too in case the On Killed function is called elsewhere
  (`self.Handle Destroyed Feedback`))

(fn `OnShot`
  (returns (ReturnValue :type Boolean))
  (if (`|EnumEquality` (`/Game/VGDC_VR/Core/BP_BaseGameState.Game State` (`/Game/VGDC_VR/Environment/Technical/BP_TunnelManager.Game State` (`/Game/VGDC_VR/Environment/Door/BP_Door.Door Manager` (`self.Owning Door`)))) "NewEnumerator0")
    (`self.Take Damage` 1)
    (return true)
    (else
      (`/Game/VGDC_VR/Blueprints/BPFL_DebugPrinting.Print Debug` "Crystal shot but game state is not in play!" true "NewEnumerator4" self)
      (return false))))

(fn `Percent to RGB`
  (params (Percent :type "Float (double-precision)"))
  (returns (R :type "Float (double-precision)") (G :type "Float (double-precision)") (B :type "Float (double-precision)"))
  (locals (Color :type Integer))
  ;[1 1 1] See color-calculations-math.py in the project root directory to see how/why this works.
  (if (<= Percent 0.5)
    (return (`/Game/VGDC_VR/Environment/BPFL_Generic.Value to Percent` (`local.Percent`) 0.0 0.5) (`/Game/VGDC_VR/Environment/BPFL_Generic.Value to Percent` (- 0.5 (`local.Percent`)) 0.0 0.5) 0.0)
    (else
      (return (`/Game/VGDC_VR/Environment/BPFL_Generic.Value to Percent` (- 1.0 (`local.Percent`)) 0.5 1.0) 0.0 (`/Game/VGDC_VR/Environment/BPFL_Generic.Value to Percent` (`local.Percent`) 0.5 1.0)))))

(fn `Take Damage`
  (params (Amount :type Integer))
  (returns (`Updated Hit Points` :type Integer) (Destroyed :type Boolean))
  ;[1 0.455 0.4152] Don't take damage if already totally rekt
  (if (> (`self.Hit Points`) 0)
    ;[0.795 0.5302 1] Update HP
    (set `self.Hit Points` (`KismetMathLibrary.Max` (- (`self.Hit Points`) (`local.Amount`))))
    (`/Game/VGDC_VR/Blueprints/BPFL_DebugPrinting.Print Debug` (`KismetStringLibrary.Concat_StrStr` "Took " (`/Game/VGDC_VR/Blueprints/BPFL_DebugPrinting.Debug Format Int` "" (`local.Amount`)) " points of damage. New HP: " (`/Game/VGDC_VR/Blueprints/BPFL_DebugPrinting.Debug Format Int` "" (`self.Hit Points`))) true "NewEnumerator4" self)
    ;[1 1 1] Feedback for the Door and Player
    (`/Game/VGDC_VR/Environment/Door/BP_Door.Recalculate Current HP` (`self.Owning Door`))
    (`self.Update Material`)
    (`self.Handle Hit Feedback`)
    ;[0.7292 1 0.4583] Destroy if HP <= 0
    (if (<= (`self.Hit Points`) 0)
      (`self.On Killed`)
      (return 0 true)
      (else
        (return (`self.Hit Points`) false)))
    (else
      (`/Game/VGDC_VR/Blueprints/BPFL_DebugPrinting.Print Debug` "Crystal shot, but HP already 0! Ignoring damage" true "NewEnumerator4" self))))

(fn `Update Material`
  ;[0.4172 0.7642 1] Change Color
  (bind (_r _g _b) (`self.Percent to RGB` (/ (`KismetMathLibrary.Conv_IntToDouble` (`self.Hit Points`)) (`KismetMathLibrary.Conv_IntToDouble` (`self.Color Maximum Health`)))))
  (`MaterialInstanceDynamic.SetVectorParameterValue` (`self.Dynamic Material`) "Color" (make `LinearColor` _r _g _b))
  ;[1 0.4583 0.4583] Turn Down Brightness
  (if (<= (`self.Hit Points`) 0)
    (`MaterialInstanceDynamic.SetScalarParameterValue` (`self.Dynamic Material`) "Brightness Percent" 0.005)
    (`MaterialInstanceDynamic.SetVectorParameterValue` :`self` (`self.Dynamic Material`) :`ParameterName` "Color")
    (else
      (`MaterialInstanceDynamic.SetScalarParameterValue` (`self.Dynamic Material`) "Brightness Percent" 1.0))))

(fn `UserConstructionScript`
  (bind _mesh (`self.Mesh`))
  (bind _returnvalue (`PrimitiveComponent.CreateDynamicMaterialInstance` _mesh 1 (`PrimitiveComponent.GetMaterial` _mesh 1)))
  (set `self.Dynamic Material` _returnvalue))