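; BP_Crystal is a shootable crystal tied to an owning door, with hit points that set its color.
; Initialization randomly picks a hit-point tier from the Difficulties map within a min/max range and applies its color through a dynamic material instance.
; Each shot decrements crystal and door hit points and updates brightness by remaining health.
; At zero it goes dark rather than being removed, pending an object pool.
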(fn `Choose Difficulty`
  (params (`Min Hit Points` :type Integer) (`Max Hit Points` :type Integer))
  (locals (`Max Index` :type Integer :default -1) (`Min Index` :type Integer :default -1))
  (bind _mesh (`self.Mesh`))
  ;[1 1 1] Make sure our parameters are valid
  (if (and (<= `Min Hit Points` `Max Hit Points`) (> `Max Hit Points` 0))
    ;[0.1129 0.7683 1] Find what the index of the highest difficulty level we can choose from without going over the Max Hit Points constraint
    (bind _keys (`BlueprintMapLibrary.Map_Keys` (`self.Difficulties`)))
    ;;[1 1 1] Set Default Max Index
    (set `local.Max Index` (- (`KismetArrayLibrary.Array_Length` _keys) 1))
    ;;[0.776 0.726 0.137] Find the min/max indices
    (for (_array_element _array_index) _keys
      (`|ExecutionSequence`
        (:`then_0`
          ;;;[1 0.08323 0] Set max difficulty index
          (if (>= (`local.Max Hit Points`) _array_element)
            (set `local.Max Index` _array_index)))
        (:`then_1`
          ;;;[0.199 1 0] Set min difficulty index
          ;;;;[1 1 1] Only set the min difficulty once!
          (if (< (`local.Min Index`) 0)
            (if (<= (`local.Min Hit Points`) _array_element)
              (set `local.Min Index` _array_index))))))
    ;[0.7746 1 0.2891] Make sure min difficulty is set (e.g. if min hp = 0, it will not have been set)
    (set `local.Min Index` (`KismetMathLibrary.Clamp` (`local.Min Index`) 0 (`local.Max Index`)))
    ;[0.2891 0.3467 1] Randomly select the difficulty level within our max difficulty constraint
    (bind _keys_2 (`BlueprintMapLibrary.Map_Keys` (`self.Difficulties`)))
    (bind _output_get (set `self.Initial Hit Points` (`|GetArrayItem` _keys_2 (`KismetMathLibrary.RandomIntegerInRange` (`local.Min Index`) (`local.Max Index`)))))
    (bind _output_get_2 (set `self.Hit Points` _output_get))
    ;[0.4855 0.1705 1] Set material color
    (bind _returnvalue (`PrimitiveComponent.CreateDynamicMaterialInstance` _mesh 0 (`PrimitiveComponent.GetMaterial` _mesh 0)))
    (`MaterialInstanceDynamic.SetVectorParameterValue` _returnvalue "Color" (`BlueprintMapLibrary.Map_Find` (`self.Difficulties`) _output_get_2))
    (else
      ;;[1 0 0] Error message if parameters are invalid
      (`KismetSystemLibrary.PrintString` (`KismetStringLibrary.Concat_StrStr` "Invalid New Crystal Difficulty! " "(" (`KismetStringLibrary.Conv_IntToString` (`local.Min Hit Points`)) ", " (`KismetStringLibrary.Conv_IntToString` (`local.Max Hit Points`)) ")") true true (struct :`R` 1.0 :`A` 1.0) 5.0)
      (return))))

(fn `Initialize Crystal`
  (params (`Min Hitpoints` :type Integer) (`Max Hitpoints` :type Integer) (`Owning Door` :type "/Game/VGDC_VR/Environment/BP_Door Object Reference"))
  (returns (Crystal :type "/Game/VGDC_VR/Environment/BP_Crystal Object Reference"))
  (`self.Choose Difficulty` `Min Hitpoints` `Max Hitpoints`)
  (set `self.Owning Door` `Owning Door`)
  (return self))

(fn `On Destroyed`
  ;[0.4855 0.1705 1] Set material color
  (bind _asmaterial_instance_dynamic (cast `MaterialInstanceDynamic` (`PrimitiveComponent.GetMaterial` (`self.Mesh`) 0)))
  (`MaterialInstanceDynamic.SetScalarParameterValue` _asmaterial_instance_dynamic "Brightness" 0.0))

(fn `OnShot`
  (returns (ReturnValue :type Boolean))
  (bind _owning_door (`self.Owning Door`))
  ;[1 0.4888 0.3075] Don't respond to shots if already destroyed
  (if (> (`self.Hit Points`) 0)
    ;[0.795 0.5302 1] Take damage
    (set `self.Hit Points` (- (`self.Hit Points`) 1))
    ;[0.1051 1 0.4063] Decrement Door HP
    (set `/Game/VGDC_VR/Environment/BP_Door.Door Hit Points` (- (`/Game/VGDC_VR/Environment/BP_Door.Door Hit Points` _owning_door) 1) _owning_door)
    ;[1 0.2243 0.5099] Update crystal brightness
    (bind _asmaterial_instance_dynamic (cast `MaterialInstanceDynamic` (`PrimitiveComponent.GetMaterial` (`self.Mesh`) 0)))
    (`MaterialInstanceDynamic.SetScalarParameterValue` _asmaterial_instance_dynamic "Brightness Percent" (/ (`KismetMathLibrary.Conv_IntToDouble` (`self.Hit Points`)) (`KismetMathLibrary.Conv_IntToDouble` (`self.Initial Hit Points`))))
    ;[0.7292 1 0.4583] Destroy if HP <= 0
    (if (<= (`self.Hit Points`) 0)
      (`self.On Destroyed`)
      (return false)
      (else
        (return false)))))

(fn `Take Damage`
  (params (Amount :type Integer))
  (returns (`Hit Points` :type Integer) (Destroyed :type Boolean))
  ;[0.795 0.5302 1] Take damage
  (bind _output_get (set `self.Hit Points` (- (`self.Hit Points`) Amount)))
  ;[0.7292 1 0.4583] Destroy if HP <= 0
  (if (<= _output_get 0)
    (`self.On Destroyed`)
    (return 0 true)
    (else
      (return (`self.Hit Points`) false))))

(fn `UserConstructionScript`)