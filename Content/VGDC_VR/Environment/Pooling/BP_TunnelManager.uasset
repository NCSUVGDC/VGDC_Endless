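; BP_TunnelManager builds the VR game's tunnel as numbered sections, each a run of hall meshes capped by a pooled crystal door.
; Curves indexed by section number set each section's length and its door's difficulty.
; GenerateNextSection moves the oldest section's hall mesh instances to the front, adds any still needed, then spawns and configures the door.
; InitializeTunnel rebuilds the starting sections, and optional Tick debug drawing visualizes segments and doors.
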(event `self.ReceiveBeginPlay`
  (`parent.ReceiveBeginPlay`)
  ;[1 1 1] Get Crystal Pooler
  (bind _pooler (`/Game/VGDC_VR/Environment/Pooling/BP_PoolerHelperMacros.Get Pooler Singleton` "/Game/VGDC_VR/Environment/Pooling/BP_CrystalPooler.BP_CrystalPooler_C")
    (:`Exec Out`
      (bind _asbp_crystal_pooler (cast `/Game/VGDC_VR/Environment/Pooling/BP_CrystalPooler` _pooler))
      (set `self.Crystal Pooler` _asbp_crystal_pooler)
      ;[1 1 1] Spawn Doors
      (if (`self.Initialize Tunnel On Begin Play`)
        (`self.Initialize Tunnel` 0)))))

(event `self.ReceiveTick`
  (params (DeltaSeconds :type "Float (single-precision)"))
  (`parent.ReceiveTick` DeltaSeconds)
  (`|ExecutionSequence`
    (:`then_0`
      ;[1 1 1] Debug Drawing
      (if (`self.Debug Draw Anything`)
        (`|ExecutionSequence`
          (:`then_0`
            (for (_array_element _array_index) (`self.Sections`)
              (`self.Debug Only First Switch` _array_index
                (:`Can Draw`
                  (set `/Game/VGDC_VR/Environment/Door/BP_Door.Debug Draw Stuff` true (`.Door_8_012F48E746953D7702307582CDC11B4F` (break `/Game/VGDC_VR/Environment/TunnelSection` _array_element)))))))
          (:`then_1`
            (for (_array_element_2 _array_index_2) (`self.Sections`)
              (`self.Debug Only First Switch` _array_index_2
                (:`Can Draw`
                  (bind (_sectionnumber _door _hallsectionindices) (break `/Game/VGDC_VR/Environment/TunnelSection` _array_element_2))
                  (for (_array_element_3 _array_index_3) _hallsectionindices
                    (`self.Debug Verbosity Check` "NewEnumerator4"
                      (:`false`
                        _)
                      (:`true`
                        (bind (_location _rotation) (`self.Get Hall Instance Transform` _array_element_3 true))
                        (bind _returnvalue (+ _location (`KismetMathLibrary.MakeVector` 0.0 0.0 (/ (`.Height` (`self.Get Hall Mesh Dimensions`)) 2.0))))
                        (`KismetSystemLibrary.DrawDebugBox` _returnvalue (`self.Get Hall Mesh Bounding Box`) (struct :`R` 0.175503 :`G` 0.59375 :`B` 0.234024 :`A` 1.0) _rotation 0.0 5.0)))
                    (`self.Debug Verbosity Check` "NewEnumerator1"
                      (:`true`
                        (if (== (- (`KismetArrayLibrary.Array_Length` _hallsectionindices) 1) _array_index_3)
                          (`KismetSystemLibrary.DrawDebugSphere` _returnvalue 60.0 10 (struct :`R` 1.0 :`G` 0.026892 :`A` 1.0) 0.0 1.0)
                          (elif (== _array_index_3 0)
                            (`KismetSystemLibrary.DrawDebugSphere` _returnvalue 60.0 10 (struct :`G` 1.0 :`B` 0.085811 :`A` 1.0) 0.0 1.0)
                            (else
                              (`KismetSystemLibrary.DrawDebugSphere` _returnvalue 35.0 8 (struct :`R` 1.0 :`G` 0.830733 :`A` 1.0) 0.0 1.0))))))))))))))))

(fn `[DEPRECATED] Respawn Doors`
  (set `self.Current Door Count DEPRECATED` 0)
  ;[1 1 1] Release every door that is active
  (while (> (`KismetArrayLibrary.Array_Length` (`self.Active Doors DEPRECATED`)) 0)
    (`self.Release Door` (`|GetArrayItem` (`self.Active Doors DEPRECATED`))))
  ;[1 1 1] Respawn ALL the doors!!
  (`self.[DEPRECATED] Spawn Doors`))

(fn `[DEPRECATED] Spawn Doors`
  (for _ (range 1 (+ (`self.Target Door Count`) 1))
    (`self.Spawn Door` 0.0)))

(fn `[EDITOR] Initialize Tunnel`
  (`self.Initialize Tunnel` 0))

(fn `[Editor] Kill Door 0`
  (locals (`Door 0` :type "/Game/VGDC_VR/Environment/Door/BP_Door Object Reference"))
  (`|ExecutionSequence`
    (:`then_0`
      ;[1 1 1] Kill all of the door's crystals so that it simulates being killed by the player
      (bind _output_get (set `local.Door 0` (`|GetArrayItem` (`self.Active Doors DEPRECATED`)))) ; See above for why this is a local variable
      (for _array_element (`/Game/VGDC_VR/Environment/Door/BP_Door.Crystals` _output_get)
        (`/Game/VGDC_VR/Environment/PowerCell/BP_Crystal.Take Damage` _array_element (`/Game/VGDC_VR/Environment/PowerCell/BP_Crystal.Hit Points` _array_element))))
    (:`then_1`
      ;[1 1 1] Door "cleanup" is handled in the Release Door function, so now just spawn another
      (`self.Spawn Door` 0.0))))

(fn `Calculate Next Hall Mesh Transform`
  (returns (ReturnValue :type "Transform Structure"))
  (locals (`Temp Offset` :type "Float (double-precision)"))
  ;[1 1 1] Store current offset for now so we can increment the offset before we return
  (set `local.Temp Offset` (`self.Next Hall Mesh Offset`))
  ;[1 1 1] Increment Next Mesh  Offset
  (set `self.Next Hall Mesh Offset` (+ (`self.Next Hall Mesh Offset`) (`self.Get Hall Mesh Dimensions`)))
  (return (`KismetMathLibrary.MakeTransform` (`KismetMathLibrary.MakeVector` (`local.Temp Offset`)))))

(fn `Generate Next Section`
  (locals (`Mesh Indices` :type "Array of Integer") (`Section Door` :type "/Game/VGDC_VR/Environment/Door/BP_Door Object Reference"))
  (bind _mesh_indices (`local.Mesh Indices`))
  ;[1 1 1] Instead of just commenting out sections, I tried collapsing sections so you can read the flow easier and isolate the parts you want to work on. Let DJ know if this is any easier or harder to read/work on! Remember, you double click these to open them, and can return to this graph by clicking the "Generate Next Section" at the top of this gridded screen space below the tabs
  (if (>= (`KismetArrayLibrary.Array_Length` (`self.Sections`)) (`self.Target Number Of Sections`))
    (for _array_element (`.HallSectionIndices_7_07018C77493389D4203F01AFAE3E9D71` (break `/Game/VGDC_VR/Environment/TunnelSection` (`|GetArrayItem` (`self.Sections`))))
      (`KismetArrayLibrary.Array_Add` (`local.Mesh Indices`) _array_element)
      (bind _returnvalue (`self.Calculate Next Hall Mesh Transform`))
      (`InstancedStaticMeshComponent.UpdateInstanceTransform` (`self.Hall Mesh`) _array_element _returnvalue false false false)))
  (for _ (range 1 (+ (- (`self.Get Section Length` -1) (`KismetArrayLibrary.Array_Length` (`local.Mesh Indices`))) 1))
    (bind _returnvalue_2 (`self.Calculate Next Hall Mesh Transform`))
    (bind _returnvalue_3 (`InstancedStaticMeshComponent.AddInstance` (`self.Hall Mesh`) _returnvalue_2))
    (`KismetArrayLibrary.Array_Add` (`local.Mesh Indices`) _returnvalue_3))
  (bind _door (`self.Spawn Door` (- (`self.Next Hall Mesh Offset`) (/ (`self.Get Hall Mesh Dimensions`) 2.0))))
  (set `local.Section Door` _door)
  (`KismetArrayLibrary.Array_Add` (`self.Sections`) (make `/Game/VGDC_VR/Environment/TunnelSection` (`self.Next Section to Generate`) (`local.Section Door`) (`local.Mesh Indices`)))
  (`/Game/VGDC_VR/Blueprints/BPFL_DebugPrinting.Print Debug` (`KismetStringLibrary.Concat_StrStr` "Generated a new hall section " (`/Game/VGDC_VR/Blueprints/BPFL_DebugPrinting.Debug Format Int` "" (`self.Next Section to Generate`)) " with door " (`KismetSystemLibrary.GetDisplayName` (`local.Section Door`)) " and " (`/Game/VGDC_VR/Blueprints/BPFL_DebugPrinting.Debug Format Int` "" (`KismetArrayLibrary.Array_Length` _mesh_indices)) " meshes (indices are " (`/Game/VGDC_VR/Blueprints/BPFL_DebugPrinting.Debug Format Int Array` "" _mesh_indices) ")") true "NewEnumerator4" self)
  ;[1 1 1] Increment Next Section!
  (`/Engine/EditorBlueprintResources/StandardMacros.IncrementInt` (`self.Next Section to Generate`)))

(fn `Get Door Difficulty`
  (params (`Section Number` :type Integer :default -1))
  (returns (Difficulty :type Integer))
  (if (< `Section Number` 0)
    ;[1 1 1] Section is negative, so use the next section's difficulty
    (return (`KismetMathLibrary.FFloor` (`CurveFloat.GetFloatValue` (`self.Door Difficulty Curve`) (`KismetMathLibrary.Conv_IntToDouble` (`self.Next Section to Generate`)))))
    (else
      ;[1 1 1] Section is non-negative, so find it's difficulty
      (return (`KismetMathLibrary.FFloor` (`CurveFloat.GetFloatValue` (`self.Door Difficulty Curve`) (`KismetMathLibrary.Conv_IntToDouble` (`local.Section Number`))))))))

(fn `Get Hall Instance Transform`
  (params (Index :type Integer) (`World Space` :type Boolean))
  (returns (Location :type "Vector Structure") (Rotation :type "Rotator Structure") (Scale :type "Vector Structure"))
  (return (.location (`InstancedStaticMeshComponent.GetInstanceTransform` (`self.Hall Mesh`) Index `World Space`)) (.rotation (`InstancedStaticMeshComponent.GetInstanceTransform` (`self.Hall Mesh`) Index `World Space`)) (.scale (`InstancedStaticMeshComponent.GetInstanceTransform` (`self.Hall Mesh`) Index `World Space`))))

(fn `Get Hall Mesh Dimensions`
  (returns (Length :type "Float (double-precision)") (Width :type "Float (double-precision)") (Height :type "Float (double-precision)"))
  (return (.x (* (`.BoxExtent` (`KismetMathLibrary.BreakBoxSphereBounds` (`StaticMesh.GetBounds` (`StaticMeshComponent.StaticMesh` (`self.Hall Mesh`))))) 2.0)) (.y (* (`.BoxExtent` (`KismetMathLibrary.BreakBoxSphereBounds` (`StaticMesh.GetBounds` (`StaticMeshComponent.StaticMesh` (`self.Hall Mesh`))))) 2.0)) (.z (* (`.BoxExtent` (`KismetMathLibrary.BreakBoxSphereBounds` (`StaticMesh.GetBounds` (`StaticMeshComponent.StaticMesh` (`self.Hall Mesh`))))) 2.0))))

(fn `Get Section Length`
  (params (`Section Number` :type Integer :default -1))
  (returns (Length :type Integer))
  (if (< `Section Number` 0)
    ;[1 1 1] Section is negative, so use the next section's length
    (return (`KismetMathLibrary.FFloor` (`CurveFloat.GetFloatValue` (`self.Hall Lengths Curve`) (`KismetMathLibrary.Conv_IntToDouble` (`self.Next Section to Generate`)))))
    (else
      ;[1 1 1] Section is non-negative, so find it's length
      (return (`KismetMathLibrary.FFloor` (`CurveFloat.GetFloatValue` (`self.Hall Lengths Curve`) (`KismetMathLibrary.Conv_IntToDouble` (`local.Section Number`))))))))

(fn `Initialize Tunnel`
  (params (`Start Section` :type Integer :default 0))
  (locals (`Current Section` :type "Float (double-precision)"))
  (bind _sections (`self.Sections`))
  (bind _returnvalue (- (+ `Start Section` (`self.Target Number Of Sections`)) 1))
  (`|ExecutionSequence`
    (:`then_0`
      (set `self.Next Section to Generate` (`local.Start Section`)))
    (:`then_1`
      (for _array_element _sections
        (`self.Release Door` (`.Door_8_012F48E746953D7702307582CDC11B4F` (break `/Game/VGDC_VR/Environment/TunnelSection` _array_element))))
      (`KismetArrayLibrary.Array_Clear` _sections))
    (:`then_2`
      (`InstancedStaticMeshComponent.ClearInstances` (`self.Hall Mesh`)))
    (:`then_3`
      (set `self.Next Hall Mesh Offset` 0.0))
    (:`then_4`
      ;[1 1 1] Loop from Start Section until we have the desired Number of Sections
      (`/Game/VGDC_VR/Blueprints/BPFL_DebugPrinting.Print Debug` (`/Game/VGDC_VR/Blueprints/BPFL_DebugPrinting.Debug Format Int Range` "Initializing tunnel segments" `Start Section` _returnvalue) true "NewEnumerator4" self)
      (for _ (range `Start Section` (+ _returnvalue 1))
        (`self.Generate Next Section`)))))

(fn `Release Door`
  (params (Door :type "/Game/VGDC_VR/Environment/Door/BP_Door Object Reference"))
  (`/Game/VGDC_VR/Environment/Door/BP_Door.Release Crystals` Door)
  (`self.activityToggle` Door)
  (`KismetArrayLibrary.Array_RemoveItem` (`self.Active Doors DEPRECATED`) (`local.Door`))
  (`/Game/VGDC_VR/Blueprints/BPFL_DebugPrinting.Print Debug` (`KismetStringLibrary.Concat_StrStr` "Releasing Door: " (`KismetSystemLibrary.GetDisplayName` (`local.Door`))) true "NewEnumerator4" self))

(fn `Spawn Door`
  (params (`X Offset` :type "Float (double-precision)"))
  (returns (Door :type "/Game/VGDC_VR/Environment/Door/BP_Door Object Reference"))
  (locals (`Spawned Door` :type "/Game/VGDC_VR/Environment/Door/BP_Door Object Reference"))
  ;[1 0.2104 0.9873] Pull door from pool
  (bind _pooledobj (`self.createActor` (+ (* (`self.GetActorForwardVector`) `X Offset`) (`self.K2_GetActorLocation`)) (`KismetMathLibrary.MakeRotator` (.roll (`self.K2_GetActorRotation`)) (.pitch (`self.K2_GetActorRotation`)) (+ (.yaw (`self.K2_GetActorRotation`)) 90.0))))
  (bind _asbp_door (cast `/Game/VGDC_VR/Environment/Door/BP_Door` _pooledobj))
  ;[0.165 0.5367 1] Perform extra setup on door
  (set `local.Spawned Door` _asbp_door)
  (set `/Game/VGDC_VR/Environment/Door/BP_Door.Door Manager` self (`local.Spawned Door`))
  (set `/Game/VGDC_VR/Environment/Door/BP_Door.Min Crystal HP` (`self.Min Crystal HP`) (`local.Spawned Door`))
  (set `/Game/VGDC_VR/Environment/Door/BP_Door.Max Crystal HP` (`self.Max Crystal HP`) (`local.Spawned Door`))
  (set `/Game/VGDC_VR/Environment/Door/BP_Door.Random Socket Selection` (`self.Randomize Crystals`) (`local.Spawned Door`))
  (set `/Game/VGDC_VR/Environment/Door/BP_Door.Section Number` (`self.Next Section to Generate`) (`local.Spawned Door`))
  (`/Game/VGDC_VR/Environment/Door/BP_Door.Initialize Door` (`local.Spawned Door`) (`self.Get Door Difficulty` -1))
  ;[1 1 1] Talk about our day & return
  (`/Game/VGDC_VR/Blueprints/BPFL_DebugPrinting.Print Debug` (`/Game/VGDC_VR/Blueprints/BPFL_DebugPrinting.Debug Format Int` "Added new door with difficulty level" (`self.Get Door Difficulty` -1)) (`self.Print Debug Messages`) "NewEnumerator4" self)
  (return (`local.Spawned Door`)))

(fn `UserConstructionScript`
  (`parent.UserConstructionScript`))