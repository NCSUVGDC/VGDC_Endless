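; BP_DoorManager is a pool manager that spawns and recycles crystal-bearing doors in the VR game.
; On BeginPlay it caches the crystal pooler singleton and can spawn a target count of pooled doors, configuring each with crystal settings and a curve-driven difficulty based on door count.
; Releasing a door frees its crystals and deactivates it.
; Editor helpers respawn all doors or simulate killing the first, and debug drawing can be limited to that door.
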(event `self.ReceiveBeginPlay`
  (`parent.ReceiveBeginPlay`)
  ;[1 1 1] Get Crystal Pooler
  (bind _pooler (`/Game/VGDC_VR/Environment/Pooling/BP_PoolerHelperMacros.Get Pooler Singleton` "/Game/VGDC_VR/Environment/Pooling/BP_CrystalPooler.BP_CrystalPooler_C")
    (:`Exec Out`
      (bind _asbp_crystal_pooler (cast `/Game/VGDC_VR/Environment/Pooling/BP_CrystalPooler` _pooler))
      (set `self.Crystal Pooler` _asbp_crystal_pooler)
      ;[1 1 1] Spawn Doors
      (if (`self.Spawn Doors On Begin Play`)
        (`self.[Editor] Respawn Doors`)))))

(event `self.ReceiveTick`
  (params (DeltaSeconds :type "Float (single-precision)"))
  (`parent.ReceiveTick` DeltaSeconds)
  (if (`self.Only Draw Debug On First Door`)
    (for (_array_element _array_index) (`self.Active Doors`)
      (set `/Game/VGDC_VR/Environment/Door/BP_Door.Debug Draw Stuff` (== _array_index 0) _array_element))))

(fn `[Editor] Kill Door 0`
  (locals (`Door 0` :type "/Game/VGDC_VR/Environment/Door/BP_Door Object Reference"))
  (`|ExecutionSequence`
    (:`then_0`
      ;[1 1 1] Kill all of the door's crystals so that it simulates being killed by the player
      (bind _output_get (set `local.Door 0` (`|GetArrayItem` (`self.Active Doors`)))) ; See above for why this is a local variable
      (for _array_element (`/Game/VGDC_VR/Environment/Door/BP_Door.Crystals` _output_get)
        (`/Game/VGDC_VR/Environment/PowerCell/BP_Crystal.Take Damage` _array_element (`/Game/VGDC_VR/Environment/PowerCell/BP_Crystal.Hit Points` _array_element))))
    (:`then_1`
      ;[1 1 1] Door "cleanup" is handled in the Release Door function, so now just spawn another
      (`self.Spawn Door`))))

(fn `[Editor] Respawn Doors`
  (set `self.Current Door Count` 0)
  ;[1 1 1] Release every door that is active
  (while (> (`KismetArrayLibrary.Array_Length` (`self.Active Doors`)) 0)
    (`self.Release Door` (`|GetArrayItem` (`self.Active Doors`))))
  ;[1 1 1] Respawn ALL the doors!!
  (`self.Spawn Doors`))

(fn `Get Current Difficulty Level`
  (returns (Difficulty :type Integer))
  (return (`KismetMathLibrary.FFloor` (`CurveFloat.GetFloatValue` (`self.Door Difficulty Curve`) (`KismetMathLibrary.Conv_IntToDouble` (`self.Current Door Count`))))))

(fn `Release Door`
  (params (Door :type "/Game/VGDC_VR/Environment/Door/BP_Door Object Reference"))
  (`/Game/VGDC_VR/Environment/Door/BP_Door.Release Crystals` Door)
  (`self.activityToggle` Door)
  (`KismetArrayLibrary.Array_RemoveItem` (`self.Active Doors`) (`local.Door`))
  (`/Game/VGDC_VR/Blueprints/BPFL_DebugPrinting.Print Debug` (`KismetStringLibrary.Concat_StrStr` "Releasing Door: " (`KismetSystemLibrary.GetDisplayName` (`local.Door`))) true "NewEnumerator4" self))

(fn `Spawn Door`
  (bind _difficulty (`self.Get Current Difficulty Level`))
  (`/Engine/EditorBlueprintResources/StandardMacros.IncrementInt` (`self.Current Door Count`)
    (:`  `
      ;[1 0.2104 0.9873] Pull door from pool
      (bind _pooledobj (`self.createActor` (+ (`KismetMathLibrary.MakeVector` 0.0 (* (`self.Current Door Count`) (`self.New Door Offset`))) (`self.K2_GetActorLocation`)) (`KismetMathLibrary.MakeRotator` (.roll (`self.K2_GetActorRotation`)) (.pitch (`self.K2_GetActorRotation`)) (+ (.yaw (`self.K2_GetActorRotation`)) 90.0))))
      (bind _asbp_door (cast `/Game/VGDC_VR/Environment/Door/BP_Door` _pooledobj))
      ;[0.165 0.5367 1] Perform extra setup on door
      (`KismetArrayLibrary.Array_Add` (`self.Active Doors`) _asbp_door)
      (set `/Game/VGDC_VR/Environment/Door/BP_Door.Door Manager` self _asbp_door)
      (set `/Game/VGDC_VR/Environment/Door/BP_Door.Min Crystal HP` (`self.Min Crystal HP`) _asbp_door)
      (set `/Game/VGDC_VR/Environment/Door/BP_Door.Max Crystal HP` (`self.Max Crystal HP`) _asbp_door)
      (set `/Game/VGDC_VR/Environment/Door/BP_Door.Random Socket Selection` (`self.Randomize Crystals`) _asbp_door)
      (set `/Game/VGDC_VR/Environment/Door/BP_Door.Difficulty Level` (`self.Current Door Count`) _asbp_door)
      (`/Game/VGDC_VR/Environment/Door/BP_Door.Initialize Door` _asbp_door _difficulty)
      (`/Game/VGDC_VR/Blueprints/BPFL_DebugPrinting.Print Debug` (`/Game/VGDC_VR/Blueprints/BPFL_DebugPrinting.Debug Format Int` "Added new door with difficulty level" _difficulty) (`self.Print Debug Messages`) "NewEnumerator4" self))))

(fn `Spawn Doors`
  (for _ (range 1 (+ (`self.Target Door Count`) 1))
    (`self.Spawn Door`)))

(fn `UserConstructionScript`
  (`parent.UserConstructionScript`)
  ;[1 1 1] Update First Door Location Arrow for debug purposes
  (`SceneComponent.K2_SetWorldLocationAndRotation` (`self.First Door Location`) (+ (`KismetMathLibrary.MakeVector` 0.0 (`self.New Door Offset`)) (`self.K2_GetActorLocation`)) (`KismetMathLibrary.MakeRotator` (.roll (`self.K2_GetActorRotation`)) (.pitch (`self.K2_GetActorRotation`)) (- (.yaw (`self.K2_GetActorRotation`)) 180.0)) false false))