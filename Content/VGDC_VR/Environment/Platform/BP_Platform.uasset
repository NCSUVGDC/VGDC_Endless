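; BP_Platform is a VR game platform that ends the game when it crashes into an intact door.
; It caches BP_BaseGameState on BeginPlay and logs a complaint if the cast fails.
; DoorCollision overlaps pass through gates for game-in-play and a BP_Door with hit points left, then set game over, or kill the door in invincibility mode.
; An editor helper forces game over, and door hits print debug messages.
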(event `self.ReceiveBeginPlay`
  ;[1 1 1] Get game state
  (bind _asbp_base_game_state (cast `/Game/VGDC_VR/Core/BP_BaseGameState` (`GameplayStatics.GetGameState`))
    (:`then`
      (set `self.Game State` _asbp_base_game_state))
    (:`CastFailed`
      (`/Game/VGDC_VR/Blueprints/BPFL_DebugPrinting.Print Debug` "Game state is not a BP_BaseGameState! Can't tell the world that the paltform has collidided!" true "NewEnumerator2" self))))

(event `self.DoorCollision.OnComponentBeginOverlap`
  (params (OverlappedComponent :type "PrimitiveComponent Object Reference") (OtherActor :type "Actor Object Reference") (OtherComp :type "PrimitiveComponent Object Reference") (OtherBodyIndex :type Integer) (bFromSweep :type Boolean) (SweepResult :type "HitResult Structure (by ref)"))
  (bind _game_state (`self.Game State`))
  (`/Engine/EditorBlueprintResources/StandardMacros.IsValid` _game_state
    (:`Is Valid`
      (if (`|EnumEquality` (`/Game/VGDC_VR/Core/BP_BaseGameState.Game State` _game_state) "NewEnumerator0")
        (bind _asbp_door (cast `/Game/VGDC_VR/Environment/Door/BP_Door` OtherActor))
        (bind _door_hit_points (`/Game/VGDC_VR/Environment/Door/BP_Door.Door Hit Points` _asbp_door))
        (if (> _door_hit_points 0)
          (`/Game/VGDC_VR/Blueprints/BPFL_DebugPrinting.Print Debug` (`KismetStringLibrary.Concat_StrStr` "Platform crashed into door \"" (`KismetSystemLibrary.GetDisplayName` _asbp_door) "\" with " (`/Game/VGDC_VR/Blueprints/BPFL_DebugPrinting.Debug Format Int` "" _door_hit_points) " HP remaining") true "NewEnumerator0" self)
          ;[1 1 1] If Invincible, just asplode the door; otherwise, game over
          (if (`self.Invincibility Mode`)
            (`/Game/VGDC_VR/Environment/Door/BP_Door.[EDITOR] Kill Door` _asbp_door)
            (else
              (`/Game/VGDC_VR/Core/BP_BaseGameState.Set Game Over` (`self.Game State`))))
          (else
            (`/Game/VGDC_VR/Blueprints/BPFL_DebugPrinting.Print Debug` (`KismetStringLibrary.Concat_StrStr` "Hit destroyed door \"" (`KismetSystemLibrary.GetDisplayName` _asbp_door) "\"" (`/Game/VGDC_VR/Blueprints/BPFL_DebugPrinting.Debug Format Int` "Reported HP Remaining" _door_hit_points)) true "NewEnumerator0" self)))))))

(fn `[EDITOR] Force Game Over`
  (`/Game/VGDC_VR/Core/BP_BaseGameState.Set Game Over` (`self.Game State`)))

(fn `UserConstructionScript`)