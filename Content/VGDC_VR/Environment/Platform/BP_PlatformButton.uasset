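; BP_PlatformButton is a shootable VR platform button that sends the player back to the HubMap level after game over.
; Every tick it reads the supplied game state and enables its mesh visibility and collision only during Game Over.
; OnShot opens HubMap in that state, and an editor helper function fires it manually for testing.
; The construction script creates a dynamic material instance for the mesh's second material slot.
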(event `/Game/VGDC_VR/Core/BPI_NeedsGameState.Set BP_BaseGameState`
  (params (State :type "/Game/VGDC_VR/Core/BP_BaseGameState Object Reference"))
  (set `self.VR Game State` State))

(event `self.ReceiveTick`
  (params (DeltaSeconds :type "Float (single-precision)"))
  (bind _returnvalue (`|EnumEquality` (`/Game/VGDC_VR/Core/BP_BaseGameState.Game State` (`self.VR Game State`)) "NewEnumerator2"))
  (`SceneComponent.SetVisibility` (`self.Mesh`) _returnvalue true)
  (`self.SetActorEnableCollision` _returnvalue))

(fn `[EDITOR] Get Shot`
  (`self.OnShot`))

(fn `OnShot`
  (returns (ReturnValue :type Boolean))
  (switch `/Game/VGDC_VR/Core/GamePlayState` (`/Game/VGDC_VR/Core/BP_BaseGameState.Game State` (`self.VR Game State`))
    (:`NewEnumerator2`
      (`/Game/VGDC_VR/Core/BPFL_DebugPrinting.Print Debug` "Platform button shot! Reloading level..." true "NewEnumerator0" self)
      (`GameplayStatics.OpenLevel` "HubMap"))))

(fn `UserConstructionScript`
  (bind _mesh (`self.Mesh`))
  (bind _returnvalue (`PrimitiveComponent.CreateDynamicMaterialInstance` _mesh 1 (`PrimitiveComponent.GetMaterial` _mesh 1)))
  (set `self.Dynamic Material` _returnvalue))