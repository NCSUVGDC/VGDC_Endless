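; BP_HubRoom is a room actor for the VR hub that can be shown or hidden as a whole.
; The construction script makes its component tree visible, then BeginPlay calls CleanUp to hide it.
; Initialize stores the given room type and shows the room again, with both functions propagating visibility from the scene root to all children.
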(event `self.ReceiveBeginPlay`
  (`self.Clean Up`))

(fn `Clean Up`
  (`SceneComponent.SetVisibility` (`self.DefaultSceneRoot`) false true))

(fn `Initialize`
  (params (`New Room Type` :type "/Game/VGDC_VR/Environment/Hub/HubRoom Enum" :default "NewEnumerator5"))
  (set `self.Room Type` `New Room Type`)
  (`SceneComponent.SetVisibility` (`self.DefaultSceneRoot`) true true))

(fn `UserConstructionScript`
  (`SceneComponent.SetVisibility` (`self.RootComponent`) true true))