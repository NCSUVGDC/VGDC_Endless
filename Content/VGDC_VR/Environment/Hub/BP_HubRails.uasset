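; BP_HubRails is the hub's railing, which extends to connect before the hub platform transition begins.
; StartConnectionSequence plays the extension sound and the skeletal mesh's extend animation at a set play rate.
; Tick polls for the animation to stop as a workaround for a blocking play, then calls StartHubPlatformTransition on the injected game state.
; OnShot only latches a warning-shot flag.
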(event `/Game/VGDC_VR/Core/BPI_NeedsGameState.Set BP_BaseGameState`
  (params (State :type "/Game/VGDC_VR/Core/BP_BaseGameState Object Reference"))
  (set `self.Game State` State))

(event `self.ReceiveTick`
  (params (DeltaSeconds :type "Float (single-precision)"))
  ;[1 1 1] I'm incredibly surpised and thoroughly disappointed that UE4 doesn't have a "Play Animation (Blocking)" or something so I don't have to do this.
  (if (`self.Has Begun Connection Sequence`)
    (if (not (`SkeletalMeshComponent.IsPlaying` (`self.SkeletalMeshComponent`)))
      (`self.On Connection Complete`))))

(fn `On Connection Complete`
  (set `self.Has Begun Connection Sequence` false)
  (`/Game/VGDC_VR/Core/BP_BaseGameState.Start Hub Platform Transition` (`self.Game State`)))

(fn `OnShot`
  (returns (ReturnValue :type Boolean))
  (if (not (`self.WarningShotHasBeenShot`))
    (set `self.WarningShotHasBeenShot` true)))

(fn `Start Connection Sequence`
  (`GameplayStatics.SpawnSoundAttached` (`self.Sound - Railing Extension`) (`self.RootComponent`))
  (`SkeletalMeshComponent.PlayAnimation` (`self.SkeletalMeshComponent`) "/Game/VGDC_VR/Environment/Hub/A_HubRails_Extend.A_HubRails_Extend" false)
  (`SkeletalMeshComponent.SetPlayRate` (`self.SkeletalMeshComponent`) (`self.AnimationPlayRate`))
  (set `self.Has Begun Connection Sequence` true))

(fn `UserConstructionScript`)