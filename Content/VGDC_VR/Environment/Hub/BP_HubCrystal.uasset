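; BP_HubCrystal is a shootable crystal in the hub that triggers rotation of the hub walls.
; OnShot swaps a mesh material and point light to green, passes its door number and reference to HubWalls.Rotate, then returns false.
; EDITORKILLME fires the same shot response by hand, and a separate DestroyHubCrystal function simply destroys the actor, with destruction effects left as a placeholder comment.
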(event `self.ReceiveBeginPlay`)

(fn `ChangeColor`
  (`PrimitiveComponent.SetMaterial` (`self.StaticMeshComponent`) 1 "/Game/VGDC_VR/Materials/Crystal_GREEN_MAT.Crystal_GREEN_MAT")
  (`LightComponent.SetLightColor` (`self.PointLight`) (struct :`R` 0.044922 :`G` 0.375 :`B` 0.04918 :`A` 1.0) true))

(fn `DestroyHubCrystal`
  ;[1 0 0.01736] Play any Crystal Destruction effects
  (`self.K2_DestroyActor`))

(fn `EDITOR_KILLME`
  (`self.OnShot`))

(fn `OnShot`
  (returns (ReturnValue :type Boolean))
  (`self.ChangeColor`)
  (`/Game/VGDC_VR/Environment/Hub/BP_HubWalls.Rotate` (`self.HubWalls`) (`self.DoorNumber`) (`self.DoorReference`))
  (return false))

(fn `UserConstructionScript`)