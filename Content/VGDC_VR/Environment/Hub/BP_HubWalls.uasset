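; Rotating hub wall actor for the VR hub that turns to line up with a requested door, then opens it.
; The construction script stacks instanced wall segments above and below the origin to TunnelHeight and positions a cap on top.
; Rotate stores the door and starts Tick-driven yaw at constant speed toward its 60-degree-step angle, choosing direction by raw yaw comparison.
; A work-in-progress approach handler initializes the game state's TunnelManager for Tunnel rooms.
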(event `/Game/VGDC_VR/Core/BPI_NeedsGameState.Set BP_BaseGameState`
  (params (State :type "/Game/VGDC_VR/Core/BP_BaseGameState Object Reference"))
  (set `self.VR Game State` State))

(event `Door Change`
  (set `self.Rotating` true))

(event `self.ReceiveTick`
  (params (DeltaSeconds :type "Float (single-precision)"))
  (if (`self.Rotating`)
    ;[0.3122 0.5972 1] Start/stop rotating if facing door
    (if (== (`self.K2_GetActorRotation`) (`KismetMathLibrary.MakeRotator` 0.0 0.0 (`self.Get Current Door Degrees (-180, 180]`)) :`ErrorTolerance` 0.1)
      ;[1 0.3281 0.4079] Done Rotating
      (set `self.Rotating` false)
      (`self.On Finished Rotating`)
      (else
        ;[0.6453 1 0.2708] Still Rotating
        (`/Engine/EditorBlueprintResources/StandardMacros.CompareFloat` (`self.Get Current Door Degrees (-180, 180]`) (.yaw (`self.K2_GetActorRotation`))
          (:`>`
            (set `self.Degrees per second` (`KismetMathLibrary.Abs` (`self.Degrees per second`))))
          (:`<`
            (bind _result (`/Engine/EditorBlueprintResources/StandardMacros.NegateFloat` (`KismetMathLibrary.Abs` (`self.Degrees per second`))) ; Make negative
              (:`  `
                (set `self.Degrees per second` _result)))))
        (`self.K2_AddActorLocalRotation` (`KismetMathLibrary.MakeRotator` 0.0 0.0 (* (`GameplayStatics.GetWorldDeltaSeconds`) (`self.Degrees per second`))))))))

(fn `On Finished Approaching Door `
  ;[1 1 1] WORK IN PROGRESS
  (switch `/Game/VGDC_VR/Environment/Hub/HubRoom` (`/Game/VGDC_VR/Environment/Hub/BP_HubDoor.Room` (`self.DoorReference`))
    (:`NewEnumerator0`
      (`/Game/VGDC_VR/Environment/Technical/BP_TunnelManager.Initialize Tunnel` (`/Game/VGDC_VR/Core/BP_BaseGameState.Tunnel Manager` (`self.VR Game State`)) false))))

(fn `On Finished Rotating`
  (`/Game/VGDC_VR/Environment/Hub/BP_HubDoor.Open` (`self.DoorReference`)))

(fn `Rotate`
  (params (DoorNumber :type Integer) (`Door Ref` :type "/Game/VGDC_VR/Environment/Hub/BP_HubDoor Object Reference"))
  (set `self.DoorNumber` DoorNumber)
  (set `self.DoorReference` `Door Ref`)
  (`self.Door Change`))

(fn `UserConstructionScript`
  (`InstancedStaticMeshComponent.ClearInstances` (`self.Mesh Levels`))
  (for _index (range (+ (`self.Tunnel Height`) 1))
    (bind _returnvalue (`KismetMathLibrary.MakeVector` 0.0 0.0 (* (`self.Get Segment Height`) (`KismetMathLibrary.Conv_IntToDouble` _index))))
    (`InstancedStaticMeshComponent.AddInstance` (`self.Mesh Levels`) (`KismetMathLibrary.MakeTransform` _returnvalue))
    (`InstancedStaticMeshComponent.AddInstance` (`self.Mesh Levels`) (`KismetMathLibrary.MakeTransform` (* _returnvalue -1.0))))
  (`SceneComponent.K2_SetRelativeLocation` (`self.Cap Mesh`) (- (`KismetMathLibrary.MakeVector` 0.0 0.0 (* (`self.Get Segment Height`) (`KismetMathLibrary.Conv_IntToDouble` (+ (`self.Tunnel Height`) 1)))) (`KismetMathLibrary.MakeVector` 0.0 0.0 (/ (`self.Get Segment Height`) 2.0))) false false))