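; BP_DemoGamePausedActor is a test actor in the VR project that displays live timing and pause state on a widget component.
; On BeginPlay it caches the component's user widget as a W_DemoGamePausedWidget.
; Every Tick it writes the delta seconds, game time in seconds and paused flag into that widget's text fields.
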(event `self.ReceiveBeginPlay`
  (bind _asw_demo_game_paused_widget (cast `/Game/VGDC_VR/Testing/W_DemoGamePausedWidget` (`WidgetComponent.GetUserWidgetObject` (`self.Widget`))))
  (set `self.WidgetObject` _asw_demo_game_paused_widget))

(event `self.ReceiveTick`
  (params (DeltaSeconds :type "Float (single-precision)"))
  (bind _widgetobject (`self.WidgetObject`))
  (`TextBlock.SetText` (`/Game/VGDC_VR/Testing/W_DemoGamePausedWidget.TickTime` _widgetobject) (`KismetTextLibrary.Conv_DoubleToText` DeltaSeconds "HalfToEven"))
  (`TextBlock.SetText` (`/Game/VGDC_VR/Testing/W_DemoGamePausedWidget.GameTime` _widgetobject) (`KismetTextLibrary.Conv_DoubleToText` (`KismetSystemLibrary.GetGameTimeInSeconds`) "HalfToEven"))
  (`TextBlock.SetText` (`/Game/VGDC_VR/Testing/W_DemoGamePausedWidget.Paused` _widgetobject) (`KismetTextLibrary.Conv_BoolToText` (`GameplayStatics.IsGamePaused`))))

(fn `UserConstructionScript`)