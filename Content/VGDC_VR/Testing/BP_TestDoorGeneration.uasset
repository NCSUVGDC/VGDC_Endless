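; Test actor that hosts in-world widget panels for exercising door generation and monitoring a target door.
; On BeginPlay it passes DoorTarget and itself to the W_TestDoorGeneration parameters widget and caches the W_TestDoorStats widget.
; Each Tick it shows the door's remaining hit points and accumulates a displayed lifespan timer while the door lives, resetting the timer to zero once hit points are depleted.
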(event `self.ReceiveBeginPlay`
  (bind _asw_test_door_generation (cast `/Game/VGDC_VR/Testing/W_TestDoorGeneration` (`WidgetComponent.GetUserWidgetObject` (`self.Params`))))
  (set `/Game/VGDC_VR/Testing/W_TestDoorGeneration.Door` (`self.Door Target`) _asw_test_door_generation)
  (set `/Game/VGDC_VR/Testing/W_TestDoorGeneration.Parent Actor` self _asw_test_door_generation)
  (bind _asw_test_door_stats (cast `/Game/VGDC_VR/Testing/W_TestDoorStats` (`WidgetComponent.GetUserWidgetObject` (`self.Stats`))))
  (set `self.Stats Widget` _asw_test_door_stats))

(event `self.ReceiveTick`
  (params (DeltaSeconds :type "Float (single-precision)"))
  (bind _door_hit_points (`/Game/VGDC_VR/Environment/Door/BP_Door.Door Hit Points` (`self.Door Target`)))
  ;[1 1 1] Update HP
  (`TextBlock.SetText` (`/Game/VGDC_VR/Testing/W_TestDoorStats.HPRemaining` (`self.Stats Widget`)) (`KismetTextLibrary.Conv_IntToText` _door_hit_points))
  (if (<= _door_hit_points 0)
    ;[1 1 1] Reset lifespan on death
    (set `self.Door Lifespan` 0.0)
    (else
      ;[1 1 1] Increase & Display Lifespan
      (bind _output_get (set `self.Door Lifespan` (+ DeltaSeconds (`self.Door Lifespan`))))
      (`TextBlock.SetText` (`/Game/VGDC_VR/Testing/W_TestDoorStats.LifespanVal` (`self.Stats Widget`)) (`KismetTextLibrary.Conv_DoubleToText` _output_get "HalfToEven")))))

(fn `UserConstructionScript`)